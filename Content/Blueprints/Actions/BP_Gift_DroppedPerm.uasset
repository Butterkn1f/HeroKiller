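; Dropped Gift actor that registers itself as a character's nearby Gift and shows this through an animated icon widget.
; On BeginPlay it looks up its Gift type from its specialty and passes it to the icon.
; Each tick it checks overlapping third-person characters, claiming the nearby slot if empty or if closer than the current Gift.
; Leaving the area clears the slot and plays the icon's off animation, if this Gift holds it.
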(event OnComponentEndOverlap(NearbyArea)
  (params (OverlappedComponent :type Primitive%20Component%20Object%20Reference) (OtherActor :type Actor%20Object%20Reference) (OtherComp :type Primitive%20Component%20Object%20Reference) (OtherBodyIndex :type Integer))
  ;[1 1 1] Upon exiting collider, if current nearby Gift is this Gift, set nearby to null
  (bind _asbp_third_person_character (Utilities|Casting|CastToBP_ThirdPersonCharacter OtherActor))
  (if (== (Variables|/Game/Blueprints/ThirdPerson/Blueprints/BP_ThirdPersonCharacter.BP_ThirdPersonCharacter_C|GetNearbyDropGift _asbp_third_person_character) self)
    (Variables|/Game/Blueprints/ThirdPerson/Blueprints/BP_ThirdPersonCharacter.BP_ThirdPersonCharacter_C|SetNearbyDropGift _asbp_third_person_character 0)
    (Default|PlayAnim (Variables|Components|GetWB%20Drop%20Gift%20Icon) false)))

(event EventBeginPlay
  (Variables|Default|SetGift%20Type (.Gift%20Type (CallFunction|GetGiftOfSpecialty (Variables|Config|GetGiftSpecialty))))
  (bind _aswb_drop_gift_icon (Utilities|Casting|CastToWB_DropGiftIcon (UserInterface|GetWidget (Variables|Default|GetIcon))))
  (bind _output_get (Variables|Components|SetWB%20Drop%20Gift%20Icon _aswb_drop_gift_icon))
  (Variables|/Game/Widgets/World/WB_DropGiftIcon.WB_DropGiftIcon_C|SetGiftType _output_get (Variables|Default|GetGift%20Type)))

(event Collision|EventActorBeginOverlap
  (params (OtherActor :type Actor%20Object%20Reference)))

(event EventTick
  (params (DeltaSeconds :type Float%20%28single-precision%29))
  (for _array_element (Collision|GetOverlappingActors (Variables|Default|GetNearbyArea) "/Game/Blueprints/ThirdPerson/Blueprints/BP_ThirdPersonCharacter.BP_ThirdPersonCharacter_C" :!class /Script/Engine.PrimitiveComponent)
    (bind _asbp_third_person_character (Utilities|Casting|CastToBP_ThirdPersonCharacter _array_element))
    (CallFunction|UpdateNearbyDroppedGift _asbp_third_person_character)))

(fn ConstructionScript)

(fn UpdateNearbyDroppedGift
  (params (ThirdPersonChar :type BP%20Third%20Person%20Character%20Object%20Reference))
  (bind _self self)
  (bind _output_get (LocalVariables|SetTPC ThirdPersonChar))
  (bind _nearbydropgift (Variables|/Game/Blueprints/ThirdPerson/Blueprints/BP_ThirdPersonCharacter.BP_ThirdPersonCharacter_C|GetNearbyDropGift _output_get)
    (:then
      (LocalVariables|SetCurrNearbyGift _nearbydropgift)
      (if (!= _nearbydropgift _self)
        ;[1 1 1] If currently nearby another Gift, check if player is closer to current Gift compared to the old one, if so, override
        (if (< (Transformation|GetDistanceTo (LocalVariables|GetTPC) self) (Transformation|GetDistanceTo (LocalVariables|GetTPC) (LocalVariables|GetCurrNearbyGift)))
          (Variables|/Game/Blueprints/ThirdPerson/Blueprints/BP_ThirdPersonCharacter.BP_ThirdPersonCharacter_C|SetNearbyDropGift (LocalVariables|GetTPC) self)
          (Default|PlayAnim (Variables|Components|GetWB%20Drop%20Gift%20Icon) true))))
    (:else
      ;[1 1 1] No nearby dropped Gift, directly set
      (Variables|/Game/Blueprints/ThirdPerson/Blueprints/BP_ThirdPersonCharacter.BP_ThirdPersonCharacter_C|SetNearbyDropGift (LocalVariables|GetTPC) _self)
      (Default|PlayAnim (Variables|Components|GetWB%20Drop%20Gift%20Icon) true))))