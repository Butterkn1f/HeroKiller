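; Gift beam actor that fires a laser toward a target actor or fallback location, damaging pawns along it.
; Tick re-aims it and line-traces to set the effect's end point and impact visual.
; A timer-driven box trace damages each BPI_Character only once, ignoring the owner.
; Damage and impact visibility are limited to a powered window within a roughly five-second timeline; the actor destroys itself when the beam effect finishes.
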(event OnSystemFinished(Beam)
  (params (PSystem :type Niagara%20Component%20Object%20Reference))
  (Actor|DestroyActor))

(event EventBeginPlay
  (Utilities|Time|SetTimerbyFunctionName 0 "UpdateDamage" 0.05)
  (Utilities|Time|SetTimerbyFunctionName 0 "UpdateDamage" 0.5 true))

(event EventTick
  (params (DeltaSeconds :type Float%20%28single-precision%29))
  (Variables|Default|SetTimeElapsed (+ (/ DeltaSeconds 5.0) (Variables|Default|GetTimeElapsed)))
  (CallFunction|UpdateBeamHit))

(fn ConstructionScript)

(fn UpdateBeamHit
  (bind _returnvalue (Transformation|GetActorLocation))
  (bind (_direction _rotation) (CallFunction|GetBeamDirectionRotation))
  (Transformation|SetActorRotation _rotation true)
  (bind _output_get (LocalVariables|SetBeamMaxEnd (+ _returnvalue (* _direction (Variables|Config|GetDistance)))))
  (bind (_outhit _returnvalue_2) (Collision|LineTraceByChannel _returnvalue _output_get "TraceTypeQuery2" false (Utilities|Array|MakeArray (Components|GetOwner)) "None"))
  (Variables|Default|SetbIsHit _returnvalue_2)
  (bind _output_get_2 (LocalVariables|SetHitLocation (.Location (Collision|BreakHitResult _outhit))))
  (bind _output_get_3 (Variables|Default|SetBeamEndLoc (Math|Vector|SelectVector _output_get_2 (LocalVariables|GetBeamMaxEnd) (Variables|Default|GetbIsHit))))
  (Effects|Components|ParticleSystem|SetVectorParameter (Variables|Default|GetBeam) "LaserEnd" _output_get_3)
  (Transformation|SetWorldLocation (Variables|Default|GetImpact) (LocalVariables|GetHitLocation) false true)
  (Rendering|SetVisibility (Variables|Default|GetImpact) (and (Variables|Default|GetbIsHit) (CallFunction|GetIsBeamPowered)) false))

(fn UpdateDamage
  (if (CallFunction|GetIsBeamPowered)
    (bind _outhits (Class|KismetSystemLibrary|BoxTraceMultiforObjects (Transformation|GetActorLocation) (Variables|Default|GetBeamEndLoc) "50.000000,50.000000,50.000000" "0, 0, 0" (Utilities|Array|MakeArray "ObjectTypeQuery3") false (Utilities|Array|MakeArray (Components|GetOwner)) "None" true))
    (for _array_element _outhits
      (if (not (Utilities|Array|ContainsItem (LocalVariables|GetHitEnemies) (.HitActor (Collision|BreakHitResult _array_element))))
        (bind _asbpi_character (Utilities|Casting|CastToBPI_Character (.HitActor (Collision|BreakHitResult _array_element))))
        (Default|TakeDamage _asbpi_character (Variables|Config|GetDamage) "NewEnumerator1")
        (Utilities|Array|AddUnique (LocalVariables|GetHitEnemies) (.HitActor (Collision|BreakHitResult _array_element)))))))

(fn GetBeamDirectionRotation
  (bind _returnvalue (Transformation|GetActorLocation))
  (bind _target (Variables|Config|GetTarget)
    (:then
      (LocalVariables|SetToLocation (Transformation|GetActorLocation _target)))
    (:else
      (LocalVariables|SetToLocation (Variables|Config|GetTargetLocation))))
  (return (Math|Vector|GetUnitDirection(Vector) _returnvalue (LocalVariables|GetToLocation)) (Math|Rotator|FindLookatRotation _returnvalue (LocalVariables|GetToLocation))))

(fn GetIsBeamPowered
  (bind _timeelapsed (Variables|Default|GetTimeElapsed))
  (return (and (>= _timeelapsed 0.05) (<= _timeelapsed 0.95))))