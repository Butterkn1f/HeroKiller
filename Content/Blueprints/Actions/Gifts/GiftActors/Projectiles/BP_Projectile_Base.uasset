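; Base projectile for gift attacks that damages characters, with an empty enemy-hit hook for children.
; It homes on a target actor or a detached invisible component at the target location, flying straight once near that point without a target.
; Overlaps filter out owner and same-owner projectiles, and dodge-ghost hits trigger perfect dodge.
; Same-element shields block it, others weaken it; wall hits spawn a chaos field, and an off-screen timer despawns it.
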(event OnComponentHit(Box)
  (params (HitComponent :type Primitive%20Component%20Object%20Reference) (OtherActor :type Actor%20Object%20Reference) (OtherComp :type Primitive%20Component%20Object%20Reference) (NormalImpulse :type Vector :default "0, 0, 0") (Hit :type Hit%20Result%20Structure%20%28by%20ref%29))
  (HitEvents|OnProjectileHitWall OtherActor OtherComp Hit))

(event OnComponentBeginOverlap(Box)
  (params (OverlappedComponent :type Primitive%20Component%20Object%20Reference) (OtherActor :type Actor%20Object%20Reference) (OtherComp :type Primitive%20Component%20Object%20Reference) (OtherBodyIndex :type Integer) (bFromSweep :type Boolean) (SweepResult :type Hit%20Result%20Structure%20%28by%20ref%29))
  ;[1 1 1] Don't want to collide with whoever owns this
  (if (!= (Components|GetOwner) OtherActor)
    (bind _asbpi_character (Utilities|Casting|CastToBPI_Character OtherActor)
      (:then
        (Utilities|OnActorHitCharacter _asbpi_character SweepResult))
      (:CastFailed
        (Utilities|Casting|CastToBP_Sera_DodgeGhost OtherActor
          (:then
            (bind _asbp_enemy (Utilities|Casting|CastToBP_Enemy (Components|GetOwner)))
            (bind _asbp_third_person_character (Utilities|Casting|CastToBP_ThirdPersonCharacter (Game|GetPlayerCharacter 0)))
            (Default|ActivatePerfectDodge _asbp_third_person_character (Variables|/Game/Blueprints/Enemy/BP_Enemy.BP_Enemy_C|GetGiftSpecialty _asbp_enemy)))
          (:CastFailed
            (Utilities|OnActorHitNonCharacter OtherActor OtherComp SweepResult)))))))

(event EventBeginPlay
  (Collision|IgnoreActorwhenMoving (Variables|Default|GetBox) (Components|GetOwner) true))

(event EventTick
  (params (DeltaSeconds :type Float%20%28single-precision%29))
  (CallFunction|DespawnOffScreen DeltaSeconds)
  (CallFunction|NearTargetCheck))

(fn ConstructionScript
  (bind _projectilemovement (Variables|Default|GetProjectileMovement))
  (bind _temptargetloc (Variables|Default|GetTempTargetLoc))
  (bind _output_get (Variables|/Script/Engine.ProjectileMovementComponent|SetInitialSpeed _projectilemovement (Variables|Config|GetSpeed)))
  (Variables|/Script/Engine.ProjectileMovementComponent|SetMaxSpeed _projectilemovement _output_get)
  (Variables|/Script/Engine.ProjectileMovementComponent|SetProjectileGravityScale _projectilemovement (Variables|Config|GetGravity))
  (Variables|Config|GetTarget
    (:then
      ;[1 1 1] If homing and has target, directly set projectile's target
      (if (Variables|Config|GetbIsHoming)
        (Variables|/Script/Engine.ProjectileMovementComponent|SetHomingTargetComponent _projectilemovement (Variables|/Script/Engine.Actor|GetRootComponent (Variables|Config|GetTarget)))
        (else
          ;[1 1 1] Else, move invis component to location of click and move projectile there
          (Transformation|DetachFromComponent (Variables|Default|GetTempTargetLoc) "KeepWorld" "KeepWorld" "KeepWorld" true :!label _label)
          (Transformation|SetWorldLocation _temptargetloc (Variables|Config|GetTargetLocation) false true)
          (bind _output_get_2 (Variables|/Script/Engine.ProjectileMovementComponent|SetHomingTargetComponent (Variables|Default|GetProjectileMovement) _temptargetloc))
          (Variables|Default|SetTargetDirection (Math|Vector|GetUnitDirection(Vector) (Transformation|GetActorLocation) (Transformation|GetWorldLocation _output_get_2))))))
    (:else
      (goto _label))))

(fn SpawnImpactParticle
  (params (Location :type Vector))
  (bind _ps_impactemitter (Variables|ConfigEffects|GetPS_ImpactEmitter)
    (:then
      (Effects|SpawnEmitteratLocation _ps_impactemitter Location))
    (:else
      (bind _ns_impactemitter (Variables|ConfigEffects|GetNS_ImpactEmitter)
        (:then
          (Niagara|SpawnSystematLocation _ns_impactemitter Location))
        (:else)))))

(fn UpdateTargetDirection
  (if (Variables|/Script/Engine.ProjectileMovementComponent|GetbIsHomingProjectile (Variables|Default|GetProjectileMovement))
    (Variables|Default|SetTargetDirection (Math|Vector|GetUnitDirection(Vector) (Transformation|GetActorLocation) (Transformation|GetActorLocation (Variables|Config|GetTarget))))
    (elif (not (< (Class|KismetMathLibrary|VectorDistanceSquared (Transformation|GetActorLocation) (Variables|Config|GetTargetLocation)) 3e+02))
      (Variables|Default|SetTargetDirection (Math|Vector|GetUnitDirection(Vector) (Transformation|GetActorLocation) (Variables|Config|GetTargetLocation))))))

(fn OnProjectileHitCharacter
  (params (Character :type BPI%20Character%20Interface) (Location :type Vector))
  (Default|TakeDamage Character (Utilities|Struct|MakeS_DamageInfo (Variables|Config|GetDamage) (Variables|Config|GetDamageResponse) (Variables|Config|GetElement) Location))
  (Impact|OnProjectileImpact Location))

(fn OnProjectileHitEnemy
  (params (Enemy :type BP%20Enemy%20Object%20Reference) (Hit :type Hit%20Result%20Structure)))

(fn OnProjectileHitWall
  (params (Actor :type Actor%20Object%20Reference) (Component :type Primitive%20Component%20Object%20Reference) (Hit :type Hit%20Result%20Structure))
  (bind (_bblockinghit _binitialoverlap _time _distance _location _impactpoint) (Collision|BreakHitResult Hit))
  (Impact|OnProjectileImpact _location)
  ;[1 1 1] Spawn chaos impact field
  (bind _returnvalue (Game|SpawnActorfromClass "/Game/Blueprints/World/Chaos/FS_MasterField.FS_MasterField_C" (Math|Transform|MakeTransform _impactpoint "0, 0, 0" "1.100000,1.000000,0.500000") "Undefined" 0 0))
  (Default|CETrigger _returnvalue))

(fn OnProjectileHitShield
  (params (Element :type E_Gift_Element%20Enum :default "NewEnumerator0") (Hit :type Hit%20Result%20Structure) (DamageReductionMultiplier :type Float%20%28double-precision%29))
  (if (Utilities|Enum|Equal(Enum) Element (Variables|Config|GetElement))
    ;[1 1 1] Collide with shield if same ele
    (HitEvents|OnProjectileHitWall 0 0 Hit)
    (else
      ;[1 1 1] Pass through shield but reduce damage
      (Variables|Config|SetDamage (* (Variables|Config|GetDamage) DamageReductionMultiplier)))))

(fn OnProjectileImpact
  (params (Location :type Vector))
  (Impact|SpawnImpactParticle Location)
  (Audio|PlaySoundatLocation (Variables|ConfigSounds|GetImpactSound) Location "0, 0, 0" 1.0 1.0 0.0 0 0 0 0)
  (Actor|DestroyActor)
  (bind _temptargetloc (Variables|Default|GetTempTargetLoc)
    (:then
      (Components|DestroyComponent _temptargetloc))
    (:else)))

(fn DespawnOffScreen
  (params (DeltaTime :type Float%20%28double-precision%29))
  ;[1 1 1] Despawn projectile after going out of screen for >3s
  (if (Rendering|IsVisible (Variables|Default|GetBox))
    (Variables|Default|SetinvisibleElapsed 0.0)
    (else
      (bind _output_get (Variables|Default|SetinvisibleElapsed (+ DeltaTime (Variables|Default|GetinvisibleElapsed))))
      (if (>= _output_get 3.0)
        (Actor|DestroyActor)
        (bind _temptargetloc (Variables|Default|GetTempTargetLoc)
          (:then
            (Components|DestroyComponent _temptargetloc))
          (:else))))))

(fn NearTargetCheck
  (bind _projectilemovement (Variables|Default|GetProjectileMovement))
  (if (and (not (Utilities|IsValid (Variables|Config|GetTarget))) (Utilities|IsValid (Variables|Default|GetTempTargetLoc)))
    (if (< (Class|KismetMathLibrary|VectorDistanceSquared (Transformation|GetActorLocation) (Transformation|GetWorldLocation (Variables|/Script/Engine.ProjectileMovementComponent|GetHomingTargetComponent (Variables|Default|GetProjectileMovement)))) 3e+02)
      (Variables|/Script/Engine.ProjectileMovementComponent|SetbIsHomingProjectile _projectilemovement false)
      (Variables|/Script/Engine.MovementComponent|SetVelocity _projectilemovement (* (Variables|Default|GetTargetDirection) (Variables|Config|GetSpeed))))))

(fn GetShouldHandleImpact
  (params (Actor :type Actor%20Object%20Reference))
  (bind _returnvalue (Utilities|GetClass Actor))
  ;[1 1 1] If actor hit is a projectile, be sure to not collide with projectiles from the same owner! (Player's projectiles can't hit other projectiles from player)
  (bind _asbp_projectile_base (Utilities|Casting|CastToBP_Projectile_Base Actor)
    (:then
      (return (!= (Components|GetOwner) (Components|GetOwner _asbp_projectile_base))))
    (:CastFailed
      (return (and (!= _returnvalue "/Game/Blueprints/Actions/Gifts/GiftActors/Fire/BP_Gift_Shield.BP_Gift_Shield_C") (!= _returnvalue "/Game/Blueprints/Actions/BP_Gift_DroppedPerm.BP_Gift_DroppedPerm_C"))))))