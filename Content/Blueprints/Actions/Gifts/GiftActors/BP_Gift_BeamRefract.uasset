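; Gift beam actor that bounces off walls by spawning progressively smaller copies of itself, up to a refraction limit.
; On a wall hit, it spawns a child at the impact point, targeted along the direction mirrored by the surface normal.
; The owner's current beam holds all children indexed by bounce, skipping existing impact points and replacing outdated segments.
; Destroying a beam destroys its tracked children.
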(event Custom|OnHitWall_Event
  (params (Hit :type Hit%20Result%20Structure))
  (CallFunction|CheckRefraction Hit))

(event Custom|OnDestroyed_Event
  (params (DestroyedActor :type Actor%20Object%20Reference))
  (for _array_element (Variables|Default|GetChildBeams)
    (Utilities|IsValid _array_element
      (:Is%20Valid
        (Actor|DestroyActor _array_element)))))

(event EventBeginPlay
  (|CallParentFunction)
  (Effects|Components|ParticleSystem|SetIntParameter (Variables|Default|GetBeam) "RefractedAmt" (Variables|Config|GetCurrRefractAmt))
  (EventDispatchers|AssignOnHitWall (delegate Custom|OnHitWall_Event))
  (Game|AssignOnDestroyed (delegate Custom|OnDestroyed_Event)))

(fn ConstructionScript
  (|CallParentFunction))

(fn CheckRefraction
  (params (Hit :type Hit%20Result%20Structure%20%28by%20ref%29))
  (LocalVariables|SetHitInfo Hit)
  (if (< (Variables|Config|GetCurrRefractAmt) (Variables|Config|GetMaxRefractAmt))
    (bind _asbpi_character (Utilities|Casting|CastToBPI_Character (Components|GetOwner)))
    (bind _beam (Default|GetCurrBeam _asbpi_character))
    (bind _asbp_gift_beam_refract (Utilities|Casting|CastToBP_Gift_BeamRefract _beam))
    (bind _output_get (LocalVariables|SetParentBeam _asbp_gift_beam_refract))
    (bind _output_get_2 (LocalVariables|SetParentChildBeams (Variables|BP_Gift_BeamRefract_C|GetChildBeams _output_get)))
    (bind _bbeamfound (CallFunction|CheckBeamExists (LocalVariables|GetHitInfo) _output_get_2))
    (if (not _bbeamfound)
      (Utilities|IsValid (Utilities|Array|Get(acopy) (LocalVariables|GetParentChildBeams) (Variables|Config|GetCurrRefractAmt))
        (:Is%20Valid
          (Utilities|Array|RemoveItem (LocalVariables|GetParentChildBeams) (Utilities|Array|Get(acopy) (LocalVariables|GetParentChildBeams) (Variables|Config|GetCurrRefractAmt)))
          (Actor|DestroyActor (Utilities|Array|Get(acopy) (LocalVariables|GetParentChildBeams) (Variables|Config|GetCurrRefractAmt))))
        (:Is%20Not%20Valid
          _))
      (bind _returnvalue (Game|SpawnActorfromClass "BP_Gift_BeamRefract_C" (Math|Transform|MakeTransform (.ImpactPoint (Collision|BreakHitResult (LocalVariables|GetHitInfo))) (Transformation|GetActorRotation) (Math|Conversions|ToVector(Float) (- 1.0 (* (+ (Variables|Config|GetCurrRefractAmt) 1) 0.3)))) "Undefined" (Components|GetOwner) (+ (Variables|Config|GetCurrRefractAmt) 1) (Variables|Config|GetMaxRefractAmt) 0 (CallFunction|GetNewTargetLoc (LocalVariables|GetHitInfo)) (Variables|Default|GetDamage) (Variables|Default|GetMaxPenetration) 0))
      (bind _output_get_3 (LocalVariables|SetSpawnedBeam _returnvalue))
      (Utilities|Array|SetArrayElem (LocalVariables|GetParentChildBeams) (Variables|Config|GetCurrRefractAmt) _output_get_3 true)
      (Variables|BP_Gift_BeamRefract_C|SetChildBeams (LocalVariables|GetParentBeam) (LocalVariables|GetParentChildBeams)))))

(fn GetNewTargetLoc
  (params (Hit :type Hit%20Result%20Structure%20%28by%20ref%29))
  (bind (_bblockinghit _binitialoverlap _time _distance _location _impactpoint _normal _impactnormal) (Collision|BreakHitResult Hit))
  (return (+ _impactpoint (Math|Vector|MirrorVectorbyNormal (.Direction (CallFunction|GetBeamDirectionRotation)) _impactnormal))))

(fn CheckBeamExists
  (params (Hit :type Hit%20Result%20Structure%20%28by%20ref%29) (Array :type Array%20of%20BP%20Gift%20Beam%20Refract%20Object%20References))
  (bind _array_element (Utilities|Array|ForEachLoopwithBreak Array :!label _label)
    (:LoopBody
      (Utilities|IsValid _array_element
        (:Is%20Valid
          (if (Utilities|Operators|EqualEqual (.ImpactPoint (Collision|BreakHitResult Hit)) (Transformation|GetActorLocation _array_element) 1.0)
            (LocalVariables|SetBeam _array_element)
            (goto _label Break)))))
    (:Completed
      (return (Utilities|IsValid (LocalVariables|GetBeam)) (LocalVariables|GetBeam)))))