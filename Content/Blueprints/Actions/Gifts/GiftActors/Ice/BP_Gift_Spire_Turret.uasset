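; Ice gift spire that acts as a turret, firing homing frostbolts at living characters around its owner.
; A looping timer starts when spawning completes and is cleared when despawn begins.
; Each tick runs a sphere overlap centered on the owner, not the spire, and filters out the dead through the character interface.
; Bolts launch from above the spire, one per target up to a bullet cap, and the owner's capsule ignores them.
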(event Custom|OnBeginDespawn_Event
  (Utilities|Time|ClearandInvalidateTimerbyHandle (Variables|Default|GetTurretTimer)))

(event Custom|OnSpawnComplete_Event
  (bind _returnvalue (Utilities|Time|SetTimerbyFunctionName 0 "SpawnFrostbolts" (Variables|Config|GetTurretInterval) true))
  (Variables|Default|SetTurretTimer _returnvalue))

(event EventBeginPlay
  (|CallParentFunction)
  (EventDispatchers|AssignOnSpawnComplete (delegate Custom|OnSpawnComplete_Event))
  (EventDispatchers|AssignOnBeginDespawn (delegate Custom|OnBeginDespawn_Event)))

(fn ConstructionScript
  (|CallParentFunction))

(fn SpawnFrostbolts
  (bind _outactors (CallFunction|GetNearbyEnemies))
  (bind _array_element (Utilities|Array|ForEachLoopwithBreak _outactors :!label _label)
    (:LoopBody
      (if (< (LocalVariables|GetUsedBullets) (Variables|Config|GetNumBullets))
        (bind _returnvalue (Game|SpawnActorfromClass "/Game/Blueprints/Actions/Gifts/GiftActors/Projectiles/BP_Projectile_Frostbolt.BP_Projectile_Frostbolt_C" (Math|Transform|MakeTransform (+ (Transformation|GetActorLocation) "0.000000,0.000000,100.000000") "0, 0, 0" "1.000000,1.000000,1.000000") "Undefined" (Components|GetOwner) 0.1 false 25.0 _array_element "0.000000,0.000000,0.000000" true "NewEnumerator2" "NewEnumerator3" "NewEnumerator2" 0))
        (Collision|IgnoreActorwhenMoving (Actor|GetComponentbyClass (Components|GetOwner) "/Script/Engine.CapsuleComponent") _returnvalue true)
        (Math|Integer|IncrementInt (LocalVariables|GetUsedBullets))
        (else
          (goto _label Break))))))

(fn GetNearbyEnemies
  (bind _foundenemies (LocalVariables|GetFoundEnemies))
  (bind _outactors (Collision|SphereOverlapActors (Transformation|GetActorLocation (Components|GetOwner)) 9e+02 (Utilities|Array|MakeArray "ObjectTypeQuery3") 0 (Utilities|Array|MakeArray (Components|GetOwner))))
  (for _array_element _outactors
    ;[1 1 1] Only add to array if not dead
    (bind _asbpi_character (Utilities|Casting|CastToBPI_Character _array_element))
    (bind _bisdead (Default|GetIsDead _asbpi_character))
    (if (not _bisdead)
      (Utilities|Array|AddUnique (LocalVariables|GetFoundEnemies) _array_element)))
  (return (> (Utilities|Array|Length _foundenemies) 0) _foundenemies))