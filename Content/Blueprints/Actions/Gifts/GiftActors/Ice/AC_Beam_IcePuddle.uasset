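; Ice puddle actor, apparently left by an ice beam gift, that makes characters slide and periodically freezes and damages them.
; Overlaps on DamageArea track characters through BPI_Character and toggle their slide state.
; A looping timer applies freeze and damage to tracked characters, skipping the puddle's owner.
; After a defrost delay, a timeline fades the dynamic material's alpha, then the puddle releases sliding characters and destroys itself.
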(event OnComponentBeginOverlap(DamageArea)
  (params (OverlappedComponent :type Primitive%20Component%20Object%20Reference) (OtherActor :type Actor%20Object%20Reference) (OtherComp :type Primitive%20Component%20Object%20Reference) (OtherBodyIndex :type Integer) (bFromSweep :type Boolean) (SweepResult :type Hit%20Result%20Structure%20%28by%20ref%29))
  (if (not (Variables|Default|GetbDeactivating))
    (bind _asbpi_character (Utilities|Casting|CastToBPI_Character OtherActor))
    (bind _returnvalue (Utilities|Array|AddUnique (Variables|Default|GetTouchedCharacters) _asbpi_character))
    (if (!= _returnvalue -1)
      (Default|BeginSlide _asbpi_character true self))))

(event OnComponentEndOverlap(DamageArea)
  (params (OverlappedComponent :type Primitive%20Component%20Object%20Reference) (OtherActor :type Actor%20Object%20Reference) (OtherComp :type Primitive%20Component%20Object%20Reference) (OtherBodyIndex :type Integer))
  (if (not (Variables|Default|GetbDeactivating))
    (bind _asbpi_character (Utilities|Casting|CastToBPI_Character OtherActor))
    (bind _returnvalue (Utilities|Array|RemoveItem (Variables|Default|GetTouchedCharacters) _asbpi_character))
    (if _returnvalue
      (Default|BeginSlide _asbpi_character false self))))

(event Custom|DefrostPuddle
  (Utilities|Time|ClearandInvalidateTimerbyHandle (Variables|Components|GetDamageTimer))
  (Variables|Default|SetbDeactivating true)
  (bind _alpha (Timeline|Timeline_Defrost PlayFromStart)
    (:Update
      (Rendering|Material|SetScalarParameterValue (Variables|Components|GetDynamicMaterial) "Alpha" (Math|Float|Lerp 1.0 0.0 _alpha) :!class /Script/Engine.MaterialInstanceDynamic))
    (:Finished
      (for _array_element (Variables|Default|GetTouchedCharacters)
        (Default|BeginSlide _array_element false self))
      (Actor|DestroyActor))))

(event EventBeginPlay
  (bind _returnvalue (Rendering|Material|CreateDynamicMaterialInstance (Variables|Default|GetPuddle) 0 "/Game/VFX/Gifts/Beam/Ice/M_Beam_Ice.M_Beam_Ice" "None" :!class /Script/Engine.PrimitiveComponent))
  (Variables|Components|SetDynamicMaterial _returnvalue)
  (bind _returnvalue_2 (Utilities|Time|SetTimerbyFunctionName 0 "DamageCharacters" (Variables|Config|GetDamageInterval) true))
  (Variables|Components|SetDamageTimer _returnvalue_2)
  (Utilities|Time|SetTimerbyEvent (EventDispatchers|CreateEvent :!event Custom|DefrostPuddle) (Variables|Config|GetDefrostTime)))

(fn ConstructionScript)

(fn DamageCharacters
  (for _array_element (Variables|Default|GetTouchedCharacters)
    (bind _asactor (Utilities|Casting|CastToActor _array_element))
    (if (!= _asactor (Components|GetOwner))
      (Default|Freeze _array_element (Variables|Config|GetFreezeDuration))
      (Default|TakeDamage _array_element (Variables|Config|GetDamage%20Amount) "NewEnumerator3"))))