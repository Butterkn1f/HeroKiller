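; Ice gift beam actor that fires a Niagara laser at a target actor or location and damages characters along it.
; Each tick it re-aims and line-traces, ending at walls or when character penetrations run out, driving the beam end and impact effect.
; A looping timer box-traces to that end during the beam's powered time window, damaging each actor once through BPI_Character.
; The actor destroys itself when the beam system finishes.
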(event OnSystemFinished(Beam)
  (params (PSystem :type Niagara%20Component%20Object%20Reference))
  (Actor|DestroyActor))

(event EventBeginPlay
  (Utilities|Time|SetTimerbyFunctionName 0 "UpdateDamage" 0.05)
  (Utilities|Time|SetTimerbyFunctionName 0 "UpdateDamage" 0.5 true)
  (Effects|Components|ParticleSystem|SetVectorParameter (Variables|Default|GetBeam) "Scale" (Class|Actor|GetActorRelativeScale3D)))

(event EventTick
  (params (DeltaSeconds :type Float%20%28single-precision%29))
  (Variables|Default|SetTimeElapsed (+ (/ DeltaSeconds 5.0) (Variables|Default|GetTimeElapsed)))
  (CallFunction|UpdateBeamHit))

(fn ConstructionScript)

(fn UpdateBeamHit
  (bind _returnvalue (Transformation|GetActorLocation))
  (bind (_direction _rotation) (CallFunction|GetBeamDirectionRotation))
  (Transformation|SetActorRotation _rotation true)
  (bind _output_get (LocalVariables|SetBeamMaxEnd (+ _returnvalue (* _direction (Variables|Config|GetDistance)))))
  (bind (_outhits _returnvalue_2) (Class|KismetSystemLibrary|LineTraceMultiforObjects _returnvalue _output_get (Utilities|Array|MakeArray "ObjectTypeQuery1" "ObjectTypeQuery3") false (Utilities|Array|MakeArray (Components|GetOwner)) "None" true))
  (bind _endhit (CallFunction|GetEndHit _outhits _returnvalue_2))
  ;[1 1 1] Set niagara params
  (bind _output_get_2 (LocalVariables|SetHitLocation (.Location (Collision|BreakHitResult _endhit))))
  (bind _output_get_3 (Variables|Default|SetBeamEndLoc (Math|Vector|SelectVector _output_get_2 (LocalVariables|GetBeamMaxEnd) (Variables|Default|GetbIsHit))))
  (Effects|Components|ParticleSystem|SetVectorParameter (Variables|Default|GetBeam) "LaserEnd" _output_get_3)
  (Transformation|SetWorldLocation (Variables|Default|GetImpact) (LocalVariables|GetHitLocation) false true)
  (Rendering|SetVisibility (Variables|Default|GetImpact) (and (Variables|Default|GetbIsHit) (CallFunction|GetIsBeamPowered)) false))

(fn UpdateDamage
  (if (CallFunction|GetIsBeamPowered)
    (bind _outhits (Class|KismetSystemLibrary|BoxTraceMultiforObjects (Transformation|GetActorLocation) (Variables|Default|GetBeamEndLoc) "50.000000,50.000000,50.000000" "0, 0, 0" (Utilities|Array|MakeArray "ObjectTypeQuery3") false (Utilities|Array|MakeArray (Components|GetOwner)) "None" true))
    (for _array_element _outhits
      (if (not (Utilities|Array|ContainsItem (LocalVariables|GetHitEnemies) (.HitActor (Collision|BreakHitResult _array_element))))
        (bind _asbpi_character (Utilities|Casting|CastToBPI_Character (.HitActor (Collision|BreakHitResult _array_element))))
        (Default|TakeDamage _asbpi_character (Utilities|Struct|MakeS_DamageInfo (Variables|Config|GetDamage) "NewEnumerator1" "NewEnumerator2" (.Location (Collision|BreakHitResult _array_element)) (Variables|Default|GetDamage%20Type)))
        (Utilities|Array|AddUnique (LocalVariables|GetHitEnemies) (.HitActor (Collision|BreakHitResult _array_element)))))))

(fn GetBeamDirectionRotation
  (bind _returnvalue (Transformation|GetActorLocation))
  (bind _target (Variables|Config|GetTarget)
    (:then
      (LocalVariables|SetToLocation (Transformation|GetActorLocation _target)))
    (:else
      (LocalVariables|SetToLocation (Variables|Config|GetTargetLocation))))
  (return (Math|Vector|GetUnitDirection(Vector) _returnvalue (LocalVariables|GetToLocation)) (Math|Rotator|FindLookatRotation _returnvalue (LocalVariables|GetToLocation))))

(fn GetIsBeamPowered
  (bind _timeelapsed (Variables|Default|GetTimeElapsed))
  (return (and (>= _timeelapsed 0.05) (<= _timeelapsed 0.95))))

(fn GetEndHit
  (params (Hit :type Array%20of%20Hit%20Result%20Structures) (bHasArrayHit :type Boolean))
  (LocalVariables|SetHits Hit)
  (if bHasArrayHit
    (LocalVariables|SetPentrationsLeft (Variables|Config|GetMaxPenetration))
    (Variables|Default|SetbIsHit false)
    (bind _array_element (Utilities|Array|ForEachLoopwithBreak (LocalVariables|GetHits) :!label _label)
      (:LoopBody
        ;[1 1 1] We don't want to immediately cut off ray by itself
        (if (not (Utilities|Operators|EqualEqual (Transformation|GetActorLocation) (.ImpactPoint (Collision|BreakHitResult _array_element)) 0.1))
          ;[1 1 1] If not enemy/player (aka wall), do not penetrate, directly cut off beam
          (bind _asbpi_character (Utilities|Casting|CastToBPI_Character (.HitActor (Collision|BreakHitResult _array_element)))
            (:then
              ;[1 1 1] If enemy/player, check if new character hit, if so, penetrate through desired characters until no penetration uses left, then set that as the end
              (bind _returnvalue (Utilities|Array|AddUnique (LocalVariables|GetHitCharacters) _asbpi_character))
              (if (!= _returnvalue -1)
                (bind _result (Math|Integer|DecrementInt (LocalVariables|GetPentrationsLeft))
                  (:%20%20
                    (if (<= _result 0)
                      (LocalVariables|SetHitEnd _array_element)
                      (Variables|Default|SetbIsHit true)
                      (goto _label Break))))))
            (:CastFailed
              (Variables|Default|SetbIsHit true)
              (bind _output_get (LocalVariables|SetHitEnd _array_element))
              (Default|CallOnHitWall _output_get)
              (goto _label Break)))))
      (:Completed
        (return (LocalVariables|GetHitEnd))))
    (else
      (Variables|Default|SetbIsHit false)
      (return ""))))