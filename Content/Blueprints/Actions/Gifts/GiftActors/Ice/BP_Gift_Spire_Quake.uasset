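; BP_Gift_Spire_Quake is an Ice gift spire actor that repeatedly emits shockwaves while it is spawned.
; When spawning completes, it starts a looping timer at the shockwave interval, and each tick calls ActivateShockwave with the freeze duration.
; The timer is cleared when despawn begins, with spawn and despawn hooks bound on BeginPlay after the parent's logic.
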(event Custom|OnBeginDespawn_Event
  (Utilities|Time|ClearandInvalidateTimerbyHandle (Variables|Default|GetShockwaveTimer)))

(event Custom|OnSpawnComplete_Event
  (bind _returnvalue (Utilities|Time|SetTimerbyEvent (delegate Custom|Event_Shockwave) (Variables|Default|GetShockwaveInterval) true))
  (Variables|Default|SetShockwaveTimer _returnvalue))

(event Custom|Event_Shockwave
  (CallFunction|ActivateShockwave (Variables|Default|GetFreezeDuration)))

(event EventBeginPlay
  (|CallParentFunction)
  (EventDispatchers|AssignOnSpawnComplete (delegate Custom|OnSpawnComplete_Event))
  (EventDispatchers|AssignOnBeginDespawn (delegate Custom|OnBeginDespawn_Event)))

(fn ConstructionScript
  (|CallParentFunction))