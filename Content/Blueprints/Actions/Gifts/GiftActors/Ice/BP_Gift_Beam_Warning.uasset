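; Telegraph actor for the ice gift beam, showing a Niagara warning beam before the damaging BP_Gift_Beam is spawned.
; Each tick it turns toward Target, or TargetLocation if none, and updates the beam's end point.
; A timer sets the warning length; completion spawns the real beam with TargetLocation and Damage, then destroys this actor.
; The line trace's penetration and wall-hit logic is disconnected, so the warning always extends to full Distance.
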(event Custom|OnWarningComplete
  (bind _returnvalue (Components|GetOwner))
  (Utilities|FlowControl|DoOnce false
    (:Completed
      (bind _returnvalue_2 (Game|SpawnActorfromClass "/Game/Blueprints/Actions/Gifts/GiftActors/Ice/BP_Gift_Beam.BP_Gift_Beam_C" (Math|Transform|MakeTransform (Transformation|GetActorLocation) "0, 0, 0" "1.000000,1.000000,1.000000") "Undefined" (Components|GetOwner) 0 (Variables|Config|GetTargetLocation) (Variables|Config|GetDamage) 1 0))
      (Actor|SetOwner _returnvalue_2 _returnvalue)
      (Collision|IgnoreActorwhenMoving (Actor|GetComponentbyClass _returnvalue "/Script/Engine.CapsuleComponent") 0 true)
      (Actor|DestroyActor))))

(event EventBeginPlay
  (Effects|Components|ParticleSystem|SetVectorParameter (Variables|Default|GetBeam) "Scale" (Class|Actor|GetActorRelativeScale3D))
  (Utilities|Time|SetTimerbyEvent (EventDispatchers|CreateEvent :!event Custom|OnWarningComplete) (Variables|Config|GetWarningDuration)))

(event EventTick
  (params (DeltaSeconds :type Float%20%28single-precision%29))
  (Variables|Default|SetTimeElapsed (+ (/ DeltaSeconds 5.0) (Variables|Default|GetTimeElapsed)))
  (CallFunction|UpdateBeamHit))

(fn ConstructionScript)

(fn UpdateBeamHit
  (bind _returnvalue (Transformation|GetActorLocation))
  (bind (_direction _rotation) (CallFunction|GetBeamDirectionRotation))
  (Transformation|SetActorRotation _rotation true)
  (bind _output_get (LocalVariables|SetBeamMaxEnd (+ _returnvalue (* _direction (Variables|Config|GetDistance)))))
  (bind (_outhits _returnvalue_2) (Class|KismetSystemLibrary|LineTraceMultiforObjects _returnvalue _output_get (Utilities|Array|MakeArray "ObjectTypeQuery1" "ObjectTypeQuery3") false (Utilities|Array|MakeArray (Components|GetOwner)) "None" true))
  (bind _endhit (CallFunction|GetEndHit _outhits _returnvalue_2))
  ;[1 1 1] Set niagara params
  (bind _output_get_2 (LocalVariables|SetHitLocation (.Location (Collision|BreakHitResult _endhit))))
  (bind _output_get_3 (Variables|Default|SetBeamEndLoc (Math|Vector|SelectVector _output_get_2 (LocalVariables|GetBeamMaxEnd) (Variables|Default|GetbIsHit))))
  (Effects|Components|ParticleSystem|SetVectorParameter (Variables|Default|GetBeam) "LaserEnd" _output_get_3))

(fn GetBeamDirectionRotation
  (bind _returnvalue (Transformation|GetActorLocation))
  (bind _target (Variables|Config|GetTarget)
    (:then
      (LocalVariables|SetToLocation (Transformation|GetActorLocation _target)))
    (:else
      (LocalVariables|SetToLocation (Variables|Config|GetTargetLocation))))
  (return (Math|Vector|GetUnitDirection(Vector) _returnvalue (LocalVariables|GetToLocation)) (Math|Rotator|FindLookatRotation _returnvalue (LocalVariables|GetToLocation))))

(fn GetIsBeamPowered
  (bind _timeelapsed (Variables|Default|GetTimeElapsed))
  (return (and (>= _timeelapsed 0.05) (<= _timeelapsed 0.95))))

(fn GetEndHit
  (params (Hit :type Array%20of%20Hit%20Result%20Structures) (bHasArrayHit :type Boolean))
  (LocalVariables|SetHits Hit)
  (Variables|Default|SetbIsHit false)
  (return ""))