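; Ice gift spire actor that rises from the ground, releases a freezing shockwave, and despawns after its active time.
; A timeline scales and lifts the spire, then plays in reverse to sink it before destroying the actor.
; Shortly after spawning, a range-scaled sphere overlap freezes and damages pawns implementing BPI_Character, ignoring the owner.
; Spawn-complete and begin-despawn calls serve as hooks for upgrade timers.
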(event Custom|TimelineEvent_SpawnSpire
  (bind _spire (Variables|Default|GetSpire))
  (bind (_direction _alpha) (Timeline|Timeline_SpawnSpire PlayFromStart)
    (:Update
      (Transformation|SetRelativeScale3D _spire (Math|Conversions|ToVector(Float) (Math|Float|Lerp 0.1 0.25 _alpha)))
      (Transformation|SetRelativeLocation _spire (Math|Vector|MakeVector 0.0 0.0 (Math|Float|Lerp -1.5e+02 -1e+01 _alpha)) false true))
    (:Finished
      (switch Utilities|FlowControl|Switch|SwitchonETimelineDirection _direction
        (:Forward
          ;[1 1 1] Begin timers for upgrades here
          (Default|CallOnSpawnComplete))
        (:Backward
          (Actor|DestroyActor))))))

(event Custom|TimelineEvent_DespawnSpire
  (bind _spire (Variables|Default|GetSpire))
  ;[1 1 1] Clear handlers for timers here
  (Default|CallOnBeginDespawn)
  (bind (_direction _alpha) (Timeline|Timeline_SpawnSpire ReverseFromEnd)
    (:Update
      (Transformation|SetRelativeScale3D _spire (Math|Conversions|ToVector(Float) (Math|Float|Lerp 0.1 0.25 _alpha)))
      (Transformation|SetRelativeLocation _spire (Math|Vector|MakeVector 0.0 0.0 (Math|Float|Lerp -1.5e+02 -1e+01 _alpha)) false true))
    (:Finished
      (switch Utilities|FlowControl|Switch|SwitchonETimelineDirection _direction
        (:Forward
          ;[1 1 1] Begin timers for upgrades here
          (Default|CallOnSpawnComplete))
        (:Backward
          (Actor|DestroyActor))))))

(event EventBeginPlay
  (bind _spire (Variables|Default|GetSpire))
  (Transformation|SetRelativeScale3D (Variables|Default|GetShockwave) (Math|Conversions|ToVector(Float) (* (Variables|Config|GetRangeMultiplier) 3.0)))
  ;[1 1 1] Initialize spire to be below ground
  (Transformation|SetRelativeScale3D _spire "0.100000,0.100000,0.100000")
  (Transformation|SetRelativeLocation _spire "0.000000,0.000000,-150.000000" false true)
  ;[1 1 1] Despawn spire after certain time
  (Utilities|Time|SetTimerbyEvent (EventDispatchers|CreateEvent :!event Custom|TimelineEvent_DespawnSpire) (Variables|Config|GetActiveTime))
  ;[1 1 1] Spawn spire animation
  (CallFunction|TimelineEventSpawnSpire)
  (Utilities|FlowControl|Delay 0.25)
  (CallFunction|ActivateShockwave 1.0))

(fn ConstructionScript)

(fn ActivateShockwave
  (params (FreezeDuration :type Float%20%28double-precision%29))
  (Components|Activation|Activate (Variables|Default|GetShockwave) true)
  (bind _outactors (Collision|SphereOverlapActors (Transformation|GetActorLocation) (* (Variables|Config|GetRangeMultiplier) 2.5e+02) (Utilities|Array|MakeArray "ObjectTypeQuery3") 0 (Utilities|Array|MakeArray (Components|GetOwner))))
  (for _array_element _outactors
    (bind _asbpi_character (Utilities|Casting|CastToBPI_Character _array_element))
    (Default|Freeze _asbpi_character FreezeDuration)
    (bind _location (Default|GetLocation _asbpi_character))
    (Default|TakeDamage _asbpi_character (Utilities|Struct|MakeS_DamageInfo (Variables|Config|GetDamage) "NewEnumerator3" "NewEnumerator2" _location (Variables|Config|GetDamage%20Type)))))