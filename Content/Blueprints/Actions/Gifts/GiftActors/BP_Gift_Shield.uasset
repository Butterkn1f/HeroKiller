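; Timed shield gift actor that reacts to enemy projectiles overlapping its sphere.
; On spawn it creates a dynamic material, dissolves in through a timeline and starts a lifetime timer.
; The destroy sequence chains two timelines, speeding up the material as a warning, then dissolving it out before destroying the actor.
; Overlapping projectiles with a different owner receive a shield-hit call with a fixed element and the sweep result.
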(event OnComponentBeginOverlap(Sphere)
  (params (OverlappedComponent :type Primitive%20Component%20Object%20Reference) (OtherActor :type Actor%20Object%20Reference) (OtherComp :type Primitive%20Component%20Object%20Reference) (OtherBodyIndex :type Integer) (bFromSweep :type Boolean) (SweepResult :type Hit%20Result%20Structure%20%28by%20ref%29))
  (bind _asbp_projectile_base (Utilities|Casting|CastToBP_Projectile_Base OtherActor))
  (if (!= (Components|GetOwner _asbp_projectile_base) (Components|GetOwner))
    (Default|OnProjectileHitShield _asbp_projectile_base "NewEnumerator0" SweepResult)))

(event Custom|SpawnShield
  (Variables|Default|SetbIsAnimating true)
  (bind _alpha (Timeline|Timeline_ShieldSpawn PlayFromStart)
    (:Update
      (Rendering|Material|SetScalarParameterValue (Variables|Components|GetMaterialInstance) "DissolveAmount" (Math|Float|Lerp 5.0 -5.0 _alpha) :!class /Script/Engine.MaterialInstanceDynamic))
    (:Finished
      (Variables|Default|SetbIsAnimating false))))

(event Custom|BeginDestroy
  (bind _materialinstance (Variables|Components|GetMaterialInstance))
  (Rendering|Material|SetScalarParameterValue _materialinstance "Destroy" 1.0 :!class /Script/Engine.MaterialInstanceDynamic)
  (bind _alpha (Timeline|Timeline_PrepareDestroy PlayFromStart)
    (:Update
      (Rendering|Material|SetScalarParameterValue _materialinstance "TimeSpeed" (Math|Float|Lerp 0.5 2.0 _alpha) :!class /Script/Engine.MaterialInstanceDynamic))
    (:Finished
      (bind _alpha_2 (Timeline|Timeline PlayFromStart)
        (:Update
          (Rendering|Material|SetScalarParameterValue (Variables|Components|GetMaterialInstance) "DissolveAmount" (Math|Float|Lerp -5.0 5.0 _alpha_2) :!class /Script/Engine.MaterialInstanceDynamic))
        (:Finished
          (Actor|DestroyActor))))))

(event EventBeginPlay
  (bind _sphere (Variables|Default|GetSphere))
  (bind _returnvalue (Rendering|Material|CreateDynamicMaterialInstance _sphere 0 (Rendering|Material|GetMaterial _sphere 0) "None" :!class /Script/Engine.PrimitiveComponent))
  (Variables|Components|SetMaterialInstance _returnvalue)
  (CallFunction|SpawnShield)
  (Utilities|Time|SetTimerbyEvent (EventDispatchers|CreateEvent :!event Custom|BeginDestroy) (Variables|Config|GetShieldTime)))

(fn ConstructionScript)