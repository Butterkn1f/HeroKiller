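; Meteor gift actor that opens a scalable ritual circle, drops a meteor diagonally, and repeatedly damages characters inside the area.
; One timeline grows the circle and triggers the fall slightly early, then starts a looping damage timer when fully open.
; Near the fall's end, it stops damage and reverses the circle timeline, destroying the actor once closed.
; Damage goes through BPI_Character to overlapping enemies and player characters, skipping the owner's class.
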(event Custom|TimelineEvent_BeginFallMeteor
  ;[1 1 1] Diagonally move meteor so it falls
  (bind _alpha (Timeline|Timeline_FallMeteor PlayFromStart)
    (:Update
      (Transformation|SetRelativeLocation (Variables|Default|GetMeteor) (Math|Vector|Lerp(Vector) (Variables|Default|GetMeteorOriginalPos) (Variables|Default|GetMeteorEndPos) _alpha) false false)
      ;[1 1 1] Close the ritual circle earlier than when timeline finishes
      (if (Math|Float|NearlyEqual(Float) _alpha 0.9 0.1)
        (Utilities|FlowControl|DoOnce false
          (:Completed
            (CallFunction|TimelineEventCloseRitual)
            (Utilities|Time|ClearandInvalidateTimerbyHandle (Variables|Default|GetDamageHandler))))))))

(event Custom|TimelineEvent_OpenRitual
  (bind _ritualcircle (Variables|Default|GetRitualCircle))
  ;[1 1 1] Expand/Shrink ritual circle
  (bind (_direction _circlesize _circlealpha) (Timeline|Timeline_OpenRitual PlayFromStart)
    (:Update
      (Niagara|SetNiagaraVariable(Float) _ritualcircle "CircleSize" (* (Variables|Config|GetAreaSizeMultiplier) _circlesize))
      (Niagara|SetNiagaraVariable(Float) _ritualcircle "CircleAlpha" _circlealpha)
      ;[1 1 1] Begin letting meteor fall slightly earlier than when timeline finishes
      (if (Math|Float|NearlyEqual(Float) _circlealpha 1.0 0.1)
        (Utilities|FlowControl|DoOnce false
          (:Completed
            (CallFunction|TimelineEventBeginFallMeteor)))))
    (:Finished
      ;[1 1 1] After finishing expanding circle, damage enemies.
      ; Upon finish shrinking, destroy entire actor
      (switch Utilities|FlowControl|Switch|SwitchonETimelineDirection _direction
        (:Forward
          (CallFunction|BeginDamaging))
        (:Backward
          (Actor|DestroyActor))))))

(event Custom|TimelineEvent_CloseRitual
  (bind _ritualcircle (Variables|Default|GetRitualCircle))
  ;[1 1 1] Expand/Shrink ritual circle
  (bind (_direction _circlesize _circlealpha) (Timeline|Timeline_OpenRitual ReverseFromEnd)
    (:Update
      (Niagara|SetNiagaraVariable(Float) _ritualcircle "CircleSize" (* (Variables|Config|GetAreaSizeMultiplier) _circlesize))
      (Niagara|SetNiagaraVariable(Float) _ritualcircle "CircleAlpha" _circlealpha)
      ;[1 1 1] Begin letting meteor fall slightly earlier than when timeline finishes
      (if (Math|Float|NearlyEqual(Float) _circlealpha 1.0 0.1)
        (Utilities|FlowControl|DoOnce false
          (:Completed
            (CallFunction|TimelineEventBeginFallMeteor)))))
    (:Finished
      ;[1 1 1] After finishing expanding circle, damage enemies.
      ; Upon finish shrinking, destroy entire actor
      (switch Utilities|FlowControl|Switch|SwitchonETimelineDirection _direction
        (:Forward
          (CallFunction|BeginDamaging))
        (:Backward
          (Actor|DestroyActor))))))

(event Custom|BeginDamaging
  (bind _returnvalue (Utilities|Time|SetTimerbyFunctionName 0 "DamageCharacters" (Variables|Config|GetDamageInterval) true))
  (Variables|Default|SetDamageHandler _returnvalue))

(event EventBeginPlay
  (bind _damagearea (Variables|Default|GetDamageArea))
  (Variables|Default|SetMeteorOriginalPos (Variables|/Script/Engine.SceneComponent|GetRelativeLocation (Variables|Default|GetMeteor)))
  (Components|Timeline|SetPlayRate (Variables|Default|GetTimeline_FallMeteor) (Variables|Config|GetMeteorSpeedMultiplier))
  (Components|Box|SetBoxExtent _damagearea (* (Variables|/Script/Engine.BoxComponent|GetBoxExtent _damagearea) (Variables|Config|GetAreaSizeMultiplier)) true)
  (CallFunction|TimelineEventOpenRitual))

(fn ConstructionScript)

(fn DamageCharacters
  (bind _damagearea (Variables|Default|GetDamageArea))
  (bind _output_get (LocalVariables|SetCharacters (Collision|GetOverlappingActors _damagearea "/Game/Blueprints/Enemy/BP_Enemy.BP_Enemy_C" :!class /Script/Engine.PrimitiveComponent)))
  (Utilities|Array|AppendArray _output_get (Collision|GetOverlappingActors _damagearea "/Game/Blueprints/ThirdPerson/Blueprints/BP_ThirdPersonCharacter.BP_ThirdPersonCharacter_C" :!class /Script/Engine.PrimitiveComponent))
  (for _array_element (LocalVariables|GetCharacters)
    (if (!= (Utilities|GetClass _array_element) (Utilities|GetClass (Components|GetOwner)))
      (bind _asbpi_character (Utilities|Casting|CastToBPI_Character _array_element))
      (Default|TakeDamage _asbpi_character (Variables|Config|GetDamagePerHit) (Variables|Default|GetDamage%20Response)))))