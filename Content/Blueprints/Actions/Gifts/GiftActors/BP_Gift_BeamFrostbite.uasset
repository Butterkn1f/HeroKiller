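; Frostbite beam gift actor that leaves ice puddles where the beam hits walls or other surfaces.
; It binds to the inherited wall-hit event and spawns AC_Beam_IcePuddle at the impact point, aligned to the surface normal.
; Puddles spawn larger on flat horizontal surfaces than on other angles.
; Spawned puddles are tracked in an array, so a hit at virtually the same point as an existing one spawns nothing.
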(event Custom|OnHitWall_Event
  (params (Hit :type Hit%20Result%20Structure))
  (CallFunction|CheckFrostbite Hit))

(event EventBeginPlay
  (|CallParentFunction)
  (EventDispatchers|AssignOnHitWall (delegate Custom|OnHitWall_Event)))

(fn ConstructionScript
  (|CallParentFunction))

(fn CheckFrostbite
  (params (Hit :type Hit%20Result%20Structure%20%28by%20ref%29))
  (bind _output_get (LocalVariables|SetHitInfo Hit))
  (bind _bpuddleexists (CallFunction|CheckExistingPuddle (.ImpactPoint (Collision|BreakHitResult _output_get))))
  (if (not _bpuddleexists)
    (bind _returnvalue (Game|SpawnActorfromClass "/Game/VFX/Gifts/Beam/Ice/AC_Beam_IcePuddle.AC_Beam_IcePuddle_C" (Math|Transform|MakeTransform (.ImpactPoint (Collision|BreakHitResult _output_get)) (Math|Rotator|MakeRotfromZ (.Normal (Collision|BreakHitResult _output_get))) (Math|Vector|SelectVector "3.000000,3.000000,3.000000" "1.500000,1.500000,1.500000" (Utilities|Operators|EqualEqual (Math|Vector|VectorGetAbs (.Normal (Collision|BreakHitResult _output_get))) "0.000000,0.000000,1.000000" 0.1))) "Undefined" (Components|GetOwner) 0))
    (Utilities|Array|AddUnique (Variables|Default|GetPuddles) _returnvalue)))

(fn CheckExistingPuddle
  (params (ImpactPoint :type Vector))
  (bind _array_element (Utilities|Array|ForEachLoopwithBreak (Variables|Default|GetPuddles) :!label _label)
    (:LoopBody
      (if (Utilities|Operators|EqualEqual (Transformation|GetActorLocation _array_element) ImpactPoint 0.1)
        (LocalVariables|SetExistingPuddle _array_element)
        (goto _label Break)))
    (:Completed
      (return (Utilities|IsValid (LocalVariables|GetExistingPuddle)) (LocalVariables|GetExistingPuddle)))))