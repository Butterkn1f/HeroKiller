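; Gift action component that fires a volley of small homing fireballs from its owning character.
; A sphere overlap around the owner finds nearby enemies, and each fireball takes a different one as its target.
; When enemies run out, remaining fireballs use the fallback from CheckProjectileTarget.
; Each spawns as a half-scale BP_Projectile_Fireball carrying damage and the gift's damage response, and the owner's capsule ignores it when moving.
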(fn SpawnGiftProjectile
  (bind _asbpi_character (Utilities|Casting|CastToBPI_Character (Components|GetOwner)))
  (LocalVariables|SetBPI%20Character _asbpi_character)
  (bind _outactors (CallFunction|GetNearbyEnemies))
  (for _index (range 0 (- (Variables|Config|GetFireballCount) 1))
    (Utilities|IsValid (Utilities|Array|Get(acopy) _outactors _index)
      (:Is%20Valid
        (Utilities|SpawnSmallFireball (LocalVariables|GetBPI%20Character) (Utilities|Array|Get(acopy) _outactors _index)))
      (:Is%20Not%20Valid
        (bind (_target _targetlocation) (CallFunction|CheckProjectileTarget (LocalVariables|GetBPI%20Character)))
        (Utilities|SpawnSmallFireball (LocalVariables|GetBPI%20Character) _target _targetlocation)))))

(fn GetNearbyEnemies
  (bind (_outactors _returnvalue) (Collision|SphereOverlapActors (Transformation|GetActorLocation (Components|GetOwner)) (Variables|Config|GetDetectionRange) (Utilities|Array|MakeArray "ObjectTypeQuery3") "/Game/Blueprints/Enemy/BP_Enemy.BP_Enemy_C"))
  (return _returnvalue _outactors))