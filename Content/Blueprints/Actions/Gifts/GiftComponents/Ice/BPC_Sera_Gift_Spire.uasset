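; Gift component for Sera's ice Spire ability, which spawns a spire actor at a floor location when cast.
; On cast, it asks the owning character through BPI_Character whether to play the cast animation and, if so, sets its cast type.
; It then spawns BP_Gift_Spire owned by the character, passing along freeze duration, damage, active time and range multiplier.
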(fn CastGift
  (bind _asbpi_character (Utilities|Casting|CastToBPI_Character (Components|GetOwner)))
  (bind _bshouldplayanim (Default|GetShouldPlayCastAnim _asbpi_character))
  (if _bshouldplayanim
    (Default|SetCastGiftType _asbpi_character (Utilities|Struct|BreakS_Gift_Type (Variables|Default|GetGiftType))))
  (CallFunction|SpawnSpire))

(fn SpawnSpire
  (Game|SpawnActorfromClass "/Game/Blueprints/Actions/Gifts/GiftActors/Ice/BP_Gift_Spire.BP_Gift_Spire_C" (Math|Transform|MakeTransform (CallFunction|GetFloorSpawnLocation) "0, 0, 0" "1.000000,1.000000,1.000000") "Undefined" (Components|GetOwner) (Variables|Details|GetFreeze%20Duration) (Variables|Default|GetDamage) (Variables|Details|GetActive%20Time) (Variables|Details|GetRange%20Multiplier) 0))