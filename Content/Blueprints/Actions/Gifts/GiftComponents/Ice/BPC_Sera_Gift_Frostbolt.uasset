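; Actor component for Sera's Frostbolt gift that spawns an ice projectile from its owning character.
; It takes the spawn transform from the owner's character interface and resolves a target and location through CheckProjectileTarget.
; The spawned BP_Projectile_Frostbolt receives damage, gift type, homing and shockwave settings, plus a short fixed freeze duration.
; The owner's capsule then ignores the projectile when moving, avoiding collision with its own shot.
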(fn SpawnGiftProjectile
  (bind _returnvalue (Components|GetOwner))
  (bind _asbpi_character (Utilities|Casting|CastToBPI_Character _returnvalue))
  (bind (_target _targetlocation) (CallFunction|CheckProjectileTarget _asbpi_character))
  (bind _spawntransform (Default|GetProjectileSpawnTransform _asbpi_character))
  (bind _returnvalue_2 (Game|SpawnActorfromClass "/Game/Blueprints/Actions/Gifts/GiftActors/Projectiles/BP_Projectile_Frostbolt.BP_Projectile_Frostbolt_C" _spawntransform "Undefined" _returnvalue 0.1 (Variables|Details|GetbHasShockwave) (Variables|Default|GetDamage) (Variables|Default|GetGiftType) _target _targetlocation (Variables|Default|GetbIsHoming) 0))
  (Collision|IgnoreActorwhenMoving (Actor|GetComponentbyClass (Components|GetOwner) "/Script/Engine.CapsuleComponent") _returnvalue_2 true))