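; Gift component for Sera's fireball that spawns either one big projectile or a volley of small ones from the owner's projectile spawn transform.
; The big fireball uses the checked projectile target and optional homing.
; Small fireballs, scaled down with reduced damage, each take a living pawn from a sphere overlap, falling back to the checked target when none remains.
; Projectiles inherit the gift's element and damage response, and the owner's capsule ignores them when moving.
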(fn SpawnGiftProjectile
  (if (Variables|Details|GetbIsSmallFireball)
    (CallFunction|SpawnSmallFireballs)
    (else
      (CallFunction|SpawnBigFireball))))

(fn GetNearbyEnemies
  (bind _foundenemies (LocalVariables|GetFoundEnemies))
  (bind _outactors (Collision|SphereOverlapActors (Transformation|GetActorLocation (Components|GetOwner)) (Variables|Config|GetDetectionRange) (Utilities|Array|MakeArray "ObjectTypeQuery3") 0 (Utilities|Array|MakeArray (Components|GetOwner))))
  (for _array_element _outactors
    ;[1 1 1] Only add to array if not dead
    (bind _asbpi_character (Utilities|Casting|CastToBPI_Character _array_element))
    (bind _bisdead (Default|GetIsDead _asbpi_character))
    (if (not _bisdead)
      (Utilities|Array|AddUnique (LocalVariables|GetFoundEnemies) _array_element)))
  (return (> (Utilities|Array|Length _foundenemies) 0) _foundenemies))

(fn SpawnBigFireball
  (bind _returnvalue (Components|GetOwner))
  (bind _gifttype (Variables|Default|GetGiftType))
  (bind (_element _damageresponse) (Utilities|Struct|BreakS_Gift_Type _gifttype))
  (bind _asbpi_character (Utilities|Casting|CastToBPI_Character _returnvalue))
  (bind (_target _targetlocation) (CallFunction|CheckProjectileTarget _asbpi_character))
  (bind _spawntransform (Default|GetProjectileSpawnTransform _asbpi_character))
  (bind _returnvalue_2 (Game|SpawnActorfromClass "/Game/Blueprints/Actions/Gifts/GiftActors/Projectiles/BP_Projectile_Fireball.BP_Projectile_Fireball_C" _spawntransform "Undefined" _returnvalue (Variables|Default|GetDamage) _target _targetlocation (Variables|Default|GetbIsHoming) _element _damageresponse 0))
  (Collision|IgnoreActorwhenMoving (Actor|GetComponentbyClass (Components|GetOwner) "/Script/Engine.CapsuleComponent") _returnvalue_2 true))

(fn SpawnSmallFireballs
  (bind _asbpi_character (Utilities|Casting|CastToBPI_Character (Components|GetOwner)))
  (LocalVariables|SetBPI%20Character _asbpi_character)
  (bind _outactors (CallFunction|GetNearbyEnemies))
  (for _index (range 0 (- (Variables|Config|GetSmallFireballCount) 1))
    (Utilities|IsValid (Utilities|Array|Get(acopy) _outactors _index)
      (:Is%20Valid
        (Utilities|SpawnSmallFireball (LocalVariables|GetBPI%20Character) (Utilities|Array|Get(acopy) _outactors _index)))
      (:Is%20Not%20Valid
        (bind (_target _targetlocation) (CallFunction|CheckProjectileTarget (LocalVariables|GetBPI%20Character)))
        (Utilities|SpawnSmallFireball (LocalVariables|GetBPI%20Character) _target _targetlocation)))))