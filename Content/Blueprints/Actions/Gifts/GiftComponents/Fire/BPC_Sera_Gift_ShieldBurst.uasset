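; Fire gift component for Sera's Shield Burst, which releases a damaging shockwave around the owning character when cast.
; CastGift runs the parent cast, then SpawnShockwave plays a scaled Niagara fire shockwave beneath the owner's location.
; A sphere overlap that ignores the owner gathers nearby actors, and those implementing BPI_Character receive ShockwaveDmg through the interface's TakeDamage.
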(fn SpawnShockwave
  (bind _asbpi_character (Utilities|Casting|CastToBPI_Character (Components|GetOwner)))
  (bind _location (Default|GetLocation _asbpi_character))
  (Niagara|SpawnSystematLocation "/Game/VFX/Gifts/Shockwave/NS_FireShockwave.NS_FireShockwave" (- _location "0.000000,0.000000,70.000000") "0, 0, 0" "5.000000,5.000000,5.000000")
  (bind _outactors (Collision|SphereOverlapActors _location 3e+02 (Utilities|Array|MakeArray "ObjectTypeQuery3" "ObjectTypeQuery2" "ObjectTypeQuery1") 0 (Utilities|Array|MakeArray (Components|GetOwner))))
  (for _array_element _outactors
    (bind _asbpi_character_2 (Utilities|Casting|CastToBPI_Character _array_element))
    (bind _location_2 (Default|GetLocation _asbpi_character_2))
    (Default|TakeDamage _asbpi_character_2 (Utilities|Struct|MakeS_DamageInfo (Variables|Config|GetShockwaveDmg) "NewEnumerator2" "NewEnumerator0" _location_2))))

(fn CastGift
  (|CallParentFunction)
  (CallFunction|SpawnShockwave))