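; Gift component for Sera's Shield ability, which surrounds the owning character with a shield actor when cast.
; CastGift sets the character's cast gift type through BPI_Character if a cast animation should play, then calls SpawnShield.
; SpawnShield destroys any current shield, spawns a scaled-up BP_Gift_Shield at the owner, attaches it and registers it as the current shield, so recasting replaces the old one.
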(fn CastGift
  (bind _asbpi_character (Utilities|Casting|CastToBPI_Character (Components|GetOwner)))
  (bind _bshouldplayanim (Default|GetShouldPlayCastAnim _asbpi_character))
  (if _bshouldplayanim
    (Default|SetCastGiftType _asbpi_character (.CastType (Utilities|Struct|BreakS_Gift_Type (Variables|Default|GetGiftType)))))
  (CallFunction|SpawnShield))

(fn SpawnShield
  (bind _returnvalue (Components|GetOwner))
  (bind _asbpi_character (Utilities|Casting|CastToBPI_Character (Components|GetOwner)))
  (bind _output_get (LocalVariables|SetCharacter _asbpi_character))
  (bind _shield (Default|GetCurrShield _asbpi_character))
  (Utilities|IsValid _shield
    (:Is%20Valid
      (Actor|DestroyActor _shield))
    (:Is%20Not%20Valid
      _))
  (bind _returnvalue_2 (Game|SpawnActorfromClass "/Game/Blueprints/Actions/Gifts/GiftActors/BP_Gift_Shield.BP_Gift_Shield_C" (Math|Transform|MakeTransform (Transformation|GetActorLocation _returnvalue) "0, 0, 0" "2.500000,2.500000,2.500000") "Undefined" _returnvalue false 0))
  (Transformation|AttachActorToActor _returnvalue_2 _returnvalue "None" "KeepWorld" "KeepWorld" "KeepWorld" true)
  (Default|SetCurrShield (LocalVariables|GetCharacter) _returnvalue_2))