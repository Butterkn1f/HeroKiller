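; Fire gift component that gives its owning character a shield, a damaging shockwave and a fireball projectile.
; CastGift sets the cast animation type, replaces any existing shield with a timed one attached to the owner, then spawns a fire shockwave that damages nearby characters via sphere overlap.
; SpawnGiftProjectile separately launches an optionally homing fireball at the checked target, ignored by the owner's capsule.
; All character access goes through BPI_Character.
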(fn SpawnGiftProjectile
  (bind _returnvalue (Components|GetOwner))
  (bind _asbpi_character (Utilities|Casting|CastToBPI_Character _returnvalue))
  (bind (_target _targetlocation) (CallFunction|CheckProjectileTarget _asbpi_character))
  (bind _spawntransform (Default|GetProjectileSpawnTransform _asbpi_character))
  (bind _returnvalue_2 (Game|SpawnActorfromClass "/Game/Blueprints/Actions/Gifts/GiftActors/Projectiles/BP_Projectile_Fireball.BP_Projectile_Fireball_C" _spawntransform "Undefined" _returnvalue (Variables|Default|GetDamage) (.DamageResponse (Utilities|Struct|BreakS_Gift_Type (Variables|Default|GetGiftType))) _target _targetlocation (Variables|Default|GetbIsHoming) 0))
  (Collision|IgnoreActorwhenMoving (Actor|GetComponentbyClass (Components|GetOwner) "/Script/Engine.CapsuleComponent") _returnvalue_2 true))

(fn CastGift
  (bind _asbpi_character (Utilities|Casting|CastToBPI_Character (Components|GetOwner)))
  (bind _bshouldplayanim (Default|GetShouldPlayCastAnim _asbpi_character))
  (if _bshouldplayanim
    (Default|SetCastGiftType _asbpi_character (Utilities|Struct|BreakS_Gift_Type (Variables|Default|GetGiftType))))
  (CallFunction|SpawnShield)
  (CallFunction|SpawnShockwave _asbpi_character))

(fn SpawnShield
  (bind _returnvalue (Components|GetOwner))
  (bind _asbpi_character (Utilities|Casting|CastToBPI_Character (Components|GetOwner)))
  (bind _output_get (LocalVariables|SetCharacter _asbpi_character))
  (bind _shield (Default|GetCurrShield _asbpi_character))
  (Utilities|IsValid _shield
    (:Is%20Valid
      (Actor|DestroyActor _shield))
    (:Is%20Not%20Valid
      _))
  (bind _returnvalue_2 (Game|SpawnActorfromClass "/Game/Blueprints/Actions/Gifts/GiftActors/BP_Gift_Shield.BP_Gift_Shield_C" (Math|Transform|MakeTransform (Transformation|GetActorLocation _returnvalue) "0, 0, 0" "2.500000,2.500000,2.500000") "Undefined" _returnvalue (Variables|Config|GetShield%20Time) 0))
  (Transformation|AttachActorToActor _returnvalue_2 _returnvalue "None" "KeepWorld" "KeepWorld" "KeepWorld" true)
  (Default|SetCurrShield (LocalVariables|GetCharacter) _returnvalue_2))

(fn SpawnShockwave
  (params (OwnerChar :type BPI%20Character%20Interface))
  (bind _location (Default|GetLocation OwnerChar))
  (Niagara|SpawnSystematLocation "/Game/VFX/Gifts/Shockwave/NS_FireShockwave.NS_FireShockwave" (- _location "0.000000,0.000000,70.000000") "0, 0, 0" "5.000000,5.000000,5.000000")
  (bind _outactors (Collision|SphereOverlapActors _location 3e+02 (Utilities|Array|MakeArray "ObjectTypeQuery3" "ObjectTypeQuery2" "ObjectTypeQuery1") 0 (Utilities|Array|MakeArray (Components|GetOwner))))
  (for _array_element _outactors
    (bind _asbpi_character (Utilities|Casting|CastToBPI_Character _array_element))
    (Default|TakeDamage _asbpi_character (Variables|Config|GetShockwaveDmg) "NewEnumerator2")))