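; Actor component for Sera's Gift shield projectile ability, which spawns a barrage-mode shield around its owning character.
; SpawnShield requires an owner implementing BPI_Character and destroys any current shield that character holds.
; It then spawns an enlarged BP_Gift_Shield at the owner's location, attaches it to the owner and registers it as the current shield through the interface.
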(fn SpawnShield
  (bind _returnvalue (Components|GetOwner))
  (bind _asbpi_character (Utilities|Casting|CastToBPI_Character (Components|GetOwner)))
  (bind _output_get (LocalVariables|SetCharacter _asbpi_character))
  (bind _shield (Default|GetCurrShield _output_get))
  (Utilities|IsValid _shield
    (:Is%20Valid
      (Actor|DestroyActor _shield))
    (:Is%20Not%20Valid
      _))
  (bind _returnvalue_2 (Game|SpawnActorfromClass :Class "/Game/Blueprints/Actions/Gifts/GiftActors/Fire/BP_Gift_Shield.BP_Gift_Shield_C" :SpawnTransform (Math|Transform|MakeTransform (Transformation|GetActorLocation _returnvalue) "0, 0, 0" "2.500000,2.500000,2.500000") :CollisionHandlingOverride "Undefined" :Owner _returnvalue :bIsBarrage true :Instigator 0))
  (Transformation|AttachActorToActor _returnvalue_2 _returnvalue "None" "KeepWorld" "KeepWorld" "KeepWorld" true)
  (Default|SetCurrShield (LocalVariables|GetCharacter) _returnvalue_2))