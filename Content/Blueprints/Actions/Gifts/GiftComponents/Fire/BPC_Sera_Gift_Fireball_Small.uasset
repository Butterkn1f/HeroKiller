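; Gift component for Sera's small fireball gift, which launches several scaled-down BP_Projectile_Fireball actors.
; A sphere overlap around the owner gathers living character pawns as "enemies", with no team check.
; Each fireball takes the next pawn found, falling back to CheckProjectileTarget when none is left.
; Projectiles spawn at the character's projectile transform with damage data and target, and the owner's capsule ignores them when moving.
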(fn SpawnGiftProjectile
  (bind _asbpi_character (Utilities|Casting|CastToBPI_Character (Components|GetOwner)))
  (LocalVariables|SetBPI%20Character _asbpi_character)
  (bind _outactors (CallFunction|GetNearbyEnemies))
  (for _index (range 0 (- (Variables|Config|GetFireballCount) 1))
    (Utilities|IsValid (Utilities|Array|Get(acopy) _outactors _index)
      (:Is%20Valid
        (Utilities|SpawnSmallFireball (LocalVariables|GetBPI%20Character) (Utilities|Array|Get(acopy) _outactors _index)))
      (:Is%20Not%20Valid
        (bind (_target _targetlocation) (CallFunction|CheckProjectileTarget (LocalVariables|GetBPI%20Character)))
        (Utilities|SpawnSmallFireball (LocalVariables|GetBPI%20Character) _target _targetlocation)))))

(fn GetNearbyEnemies
  (bind _foundenemies (LocalVariables|GetFoundEnemies))
  (bind _outactors (Collision|SphereOverlapActors (Transformation|GetActorLocation (Components|GetOwner)) (Variables|Config|GetDetectionRange) (Utilities|Array|MakeArray "ObjectTypeQuery3") 0 (Utilities|Array|MakeArray (Components|GetOwner))))
  (for _array_element _outactors
    ;[1 1 1] Only add to array if not dead
    (bind _asbpi_character (Utilities|Casting|CastToBPI_Character _array_element))
    (bind _bisdead (Default|GetIsDead _asbpi_character))
    (if (not _bisdead)
      (Utilities|Array|AddUnique (LocalVariables|GetFoundEnemies) _array_element)))
  (return (> (Utilities|Array|Length _foundenemies) 0) _foundenemies))