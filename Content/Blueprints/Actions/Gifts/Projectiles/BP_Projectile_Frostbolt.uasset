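; Frostbolt gift projectile that freezes the character it hits for a set duration.
; When its shockwave option is on and the target is an enemy, it spawns an ice shockwave effect at the target's feet.
; It then runs a sphere overlap around that enemy and sends a freeze message to every enemy in range.
; All logic extends the parent projectile's character-hit handler.
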(event EventBeginPlay
  (|CallParentFunction))

(event Collision|EventActorBeginOverlap
  (params (OtherActor :type Actor%20Object%20Reference))
  (|CallParentFunction OtherActor) ; This node is disabled and will not be called.\nDrag off pins to build functionality.
)

(event EventTick
  (params (DeltaSeconds :type Float%20%28single-precision%29))
  (|CallParentFunction DeltaSeconds) ; This node is disabled and will not be called.\nDrag off pins to build functionality.
)

(fn ConstructionScript
  (|CallParentFunction))

(fn OnProjectileHitCharacter
  (params (Character :type BPI%20Character%20Interface) (Location :type Vector :default "0, 0, 0"))
  (|CallParentFunction Character Location)
  (Default|Freeze Character (Variables|Config|GetFreezeDuration))
  (if (Variables|Config|GetbHasShockwave)
    (Utilities|Casting|CastToBP_Enemy Character)
    (bind _location (Default|GetLocation Character))
    (Niagara|SpawnSystematLocation "/Game/VFX/Gifts/Shockwave/NS_IceShockwave.NS_IceShockwave" (- _location "0.000000,0.000000,80.000000") "0, 0, 0" "3.000000,3.000000,3.000000")
    (bind _outactors (Collision|SphereOverlapActors _location 4e+02 (Utilities|Array|MakeArray "ObjectTypeQuery3") "/Game/Blueprints/Enemy/BP_Enemy.BP_Enemy_C"))
    (for _array_element _outactors
      (Class|BPICharacter|Freeze(Message) _array_element (Variables|Config|GetFreezeDuration)))))