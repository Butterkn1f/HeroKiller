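; Fireball projectile Blueprint for a gift action, relying on its parent class for nearly all behavior.
; On BeginPlay it runs the parent logic, then binds to the enemy-hit event.
; When the projectile hits an enemy, it calls OnProjectileImpact at the hit location.
; Tick, overlap and construction add no logic of their own.
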(event Custom|OnProjectileHitEnemy_Event
  (params (Enemy :type BP%20Enemy%20Object%20Reference) (Hit :type Hit%20Result%20Structure))
  ;[1 1 1] No special functionality needed
  (CallFunction|OnProjectileImpact (.Location (Collision|BreakHitResult Hit))))

(event EventBeginPlay
  (|CallParentFunction)
  (EventDispatchers|AssignOnProjectileHitEnemy (delegate Custom|OnProjectileHitEnemy_Event)))

(event Collision|EventActorBeginOverlap
  (params (OtherActor :type Actor%20Object%20Reference))
  (|CallParentFunction OtherActor) ; This node is disabled and will not be called.\nDrag off pins to build functionality.
)

(event EventTick
  (params (DeltaSeconds :type Float%20%28single-precision%29))
  (|CallParentFunction DeltaSeconds) ; This node is disabled and will not be called.\nDrag off pins to build functionality.
)

(fn ConstructionScript
  (|CallParentFunction))