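; Base projectile actor for gift actions that damages overlapped characters other than its owner and raises enemy-hit and wall-hit notifications.
; Construction configures speed, gravity and optional homing, while a timeline lerps velocity toward the homing target or a fixed location, halting near the latter.
; Blocking hits spawn a Cascade or Niagara effect with sound and destroy it, whereas overlaps do not.
; It also despawns after several seconds off screen.
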(event OnComponentHit(Box)
  (params (HitComponent :type Primitive%20Component%20Object%20Reference) (OtherActor :type Actor%20Object%20Reference) (OtherComp :type Primitive%20Component%20Object%20Reference) (NormalImpulse :type Vector :default "0, 0, 0") (Hit :type Hit%20Result%20Structure%20%28by%20ref%29))
  (Default|CallOnProjectileHitWall OtherActor Hit)
  (CallFunction|OnProjectileImpact (.Location (Collision|BreakHitResult Hit))))

(event OnComponentBeginOverlap(Box)
  (params (OverlappedComponent :type Primitive%20Component%20Object%20Reference) (OtherActor :type Actor%20Object%20Reference) (OtherComp :type Primitive%20Component%20Object%20Reference) (OtherBodyIndex :type Integer) (bFromSweep :type Boolean) (SweepResult :type Hit%20Result%20Structure%20%28by%20ref%29))
  (if (!= (Components|GetOwner) OtherActor)
    (bind _asbpi_character (Utilities|Casting|CastToBPI_Character OtherActor))
    (Default|TakeDamage _asbpi_character (Variables|Config|GetDamage) (Variables|Config|GetDamageResponse))
    (bind _asbp_enemy (Utilities|Casting|CastToBP_Enemy OtherActor))
    (Default|CallOnProjectileHitEnemy _asbp_enemy SweepResult)))

(event Custom|TimelineEvent_RotateToTarget
  (bind _alpha (Timeline|Timeline_Rotate PlayFromStart)
    (:Update
      (CallFunction|UpdateTargetDirection)
      (Variables|/Script/Engine.MovementComponent|SetVelocity (Variables|Default|GetProjectileMovement) (Math|Vector|Lerp(Vector) (Variables|/Script/Engine.MovementComponent|GetVelocity (Variables|Default|GetProjectileMovement)) (* (Variables|Default|GetTargetDirection) (Variables|Config|GetSpeed)) _alpha)))))

(event EventBeginPlay
  (Collision|IgnoreActorwhenMoving (Variables|Default|GetBox) (Components|GetOwner) true)
  (CallFunction|TimelineEventRotatetoTarget))

(event EventTick
  (params (DeltaSeconds :type Float%20%28single-precision%29))
  ;[1 1 1] Despawn projectile after going out of screen for >3s
  (if (Rendering|IsVisible (Variables|Default|GetBox))
    (Variables|Default|SetinvisibleElapsed 0.0)
    (else
      (bind _output_get (Variables|Default|SetinvisibleElapsed (+ DeltaSeconds (Variables|Default|GetinvisibleElapsed))))
      (if (>= _output_get 3.0)
        (Actor|DestroyActor)))))

(fn ConstructionScript
  (bind _projectilemovement (Variables|Default|GetProjectileMovement))
  (bind _output_get (Variables|/Script/Engine.ProjectileMovementComponent|SetInitialSpeed _projectilemovement (Variables|Config|GetSpeed)))
  (Variables|/Script/Engine.ProjectileMovementComponent|SetMaxSpeed _projectilemovement _output_get)
  (Variables|/Script/Engine.ProjectileMovementComponent|SetProjectileGravityScale _projectilemovement (Variables|Config|GetGravity))
  (Variables|Config|GetTarget
    (:then
      (if (Variables|Config|GetbIsHoming)
        (Variables|/Script/Engine.ProjectileMovementComponent|SetbIsHomingProjectile _projectilemovement true)
        (Variables|/Script/Engine.ProjectileMovementComponent|SetHomingTargetComponent _projectilemovement (Variables|/Script/Engine.Actor|GetRootComponent (Variables|Config|GetTarget)))))
    (:else)))

(fn SpawnImpactParticle
  (params (Location :type Vector))
  (bind _ps_impactemitter (Variables|ConfigEffects|GetPS_ImpactEmitter)
    (:then
      (Effects|SpawnEmitteratLocation _ps_impactemitter Location))
    (:else
      (bind _ns_impactemitter (Variables|ConfigEffects|GetNS_ImpactEmitter)
        (:then
          (Niagara|SpawnSystematLocation _ns_impactemitter Location))
        (:else)))))

(fn UpdateTargetDirection
  (if (Variables|/Script/Engine.ProjectileMovementComponent|GetbIsHomingProjectile (Variables|Default|GetProjectileMovement))
    (Variables|Default|SetTargetDirection (Math|Vector|GetUnitDirection(Vector) (Transformation|GetActorLocation) (Transformation|GetActorLocation (Variables|Config|GetTarget))))
    (elif (< (Class|KismetMathLibrary|VectorDistanceSquared (Transformation|GetActorLocation) (Variables|Config|GetTargetLocation)) 2e+02)
      ;[1 1 1] Stop updating velocity & direction once near/past target
      (Audio|Components|Audio|Stop (Variables|Default|GetTimeline_Rotate))
      (else
        (Variables|Default|SetTargetDirection (Math|Vector|GetUnitDirection(Vector) (Transformation|GetActorLocation) (Variables|Config|GetTargetLocation)))))))

(fn OnProjectileImpact
  (params (Location :type Vector))
  (CallFunction|SpawnImpactParticle Location)
  (Audio|PlaySoundatLocation (Variables|ConfigSounds|GetImpactSound) Location "0, 0, 0" 1.0 1.0 0.0 0 0 0 0)
  (Actor|DestroyActor))