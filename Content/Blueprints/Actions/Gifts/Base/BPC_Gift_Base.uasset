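; Base actor component for Gifts, castable abilities that fire projectiles from an owning character.
; CastGift uses BPI_Character to either hand itself and its cast type to the character to fire after the cast animation, or call the empty SpawnGiftProjectile directly.
; CheckProjectileTarget picks the target actor for valid homing shots, otherwise a location.
; Temporary use decrements uses and reports depletion, permanent use returns mana cost, and DestroyGift removes the component after a short delay.
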(event Custom|DestroyGift
  (Utilities|FlowControl|Delay 0.5)
  (Components|DestroyComponent))

(fn CastGift
  (bind _asbpi_character (Utilities|Casting|CastToBPI_Character (Components|GetOwner)))
  (bind _bshouldplayanim (Default|GetShouldPlayCastAnim _asbpi_character))
  (if _bshouldplayanim
    ;[1 1 1] Wait for anim to finish playing before firing gift
    (Default|SetCastGiftType _asbpi_character (.CastType (Utilities|Struct|BreakS_Gift_Type (Variables|Details|GetGiftType))))
    (Default|SetCurrFiringGift _asbpi_character self)
    (else
      ;[1 1 1] Directly fire Gift
      (CallFunction|SpawnGiftProjectile))))

(fn SpawnGiftProjectile)

(fn CheckProjectileTarget
  (params (BPI%20Character :type BPI%20Character%20Interface))
  ;[1 1 1] Based on whether homing, return different types of target
  (bind (_target _targetlocation) (Default|GetProjectileTarget BPI%20Character))
  (if (Variables|Details|GetbIsHoming)
    (Utilities|IsValid _target
      (:Is%20Valid
        (return _target "0, 0, 0"))
      (:Is%20Not%20Valid
        _)))
  (return 0 _targetlocation))

(fn UseGiftTemp
  (CallFunction|CastGift)
  (bind _output_get (Variables|Details|Set_usesLeft (- (Variables|Details|Get_usesLeft) 1)))
  (return (== _output_get 0)))

(fn UseGiftPerm
  (CallFunction|CastGift)
  (return (Variables|Details|Get_manaCost)))