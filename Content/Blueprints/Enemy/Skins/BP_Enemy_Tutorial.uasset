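; Tutorial enemy Blueprint that can trigger dialogue when it dies, in addition to the parent death behavior.
; On death, a DoOnce gate switches on ShowDialogueType, either showing dialogue after a short delay or first checking that every enemy in KillEnemiesBeforeDialogue is dead.
; Non-empty dialogue lists are passed to InsertNewDialogues with the third-person character, auto-advance and override settings.
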(event EventOnDead
  (|CallParentFunction)
  (Utilities|FlowControl|DoOnce false
    (:Completed
      (switch int (Variables|Config|GetShowDialogueType)
        (:1
          (Utilities|FlowControl|Delay 2.0)
          (CallFunction|ShowDialogues))
        (:2
          (Utilities|FlowControl|Delay 2.0)
          (CallFunction|OnKillEnemyinGroup))))))

(fn ConstructionScript
  (|CallParentFunction))

(fn OnKillEnemyinGroup
  (bind _array_element (Utilities|Array|ForEachLoopwithBreak (Variables|Config|GetKillEnemiesBeforeDialogue) :!label _label)
    (:LoopBody
      (bind _bisdead (Default|GetIsDead _array_element))
      (if (not _bisdead)
        (LocalVariables|SetbNotAllDead true)
        (goto _label Break)))
    (:Completed
      ;[1 1 1] Show dialogue once all enemies in group are dead.
      (if (not (LocalVariables|GetbNotAllDead))
        (CallFunction|ShowDialogues)))))

(fn ShowDialogues
  (bind _dialogues (Variables|Config|GetDialogues))
  (if (Utilities|Array|IsNotEmpty _dialogues)
    (CallFunction|InsertNewDialogues (Variables|Default|GetTPC) _dialogues (Variables|Config|GetbAutoAdvance) (Variables|Config|GetbOverridePrevious))))