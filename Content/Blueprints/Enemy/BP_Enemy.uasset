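; Enemy character that casts fireball or frostbolt Gifts at the player by element, and on death ragdolls, drops its Gift and notifies the player.
; BPCCharacter holds health and state; damage feeds it, the player's damage window, AI damage sensing and the HP widget.
; A melee sphere trace damages the player or triggers perfect dodge on dodge ghosts.
; Freeze zeroes CustomTimeDilation and drives dynamic material FreezeAmount, with a dilation-immune timeline for thawing.
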(event OnHit(BPC_Character)
  (Animation|Montage|PlayMontage (Variables|Character|GetMesh) "/Game/Characters/Enemy/Animations/AM_Enemy_Hit.AM_Enemy_Hit"
    (:then
      (Variables|/Game/Blueprints/Common/BPC_Character.BPC_Character_C|SetbIsHit (Variables|Default|GetBPC_Character) false))))

(event OnBeginCursorOver(Mesh)
  (params (TouchedComponent :type Primitive%20Component%20Object%20Reference))
  (bind _tpc (Variables|Default|GetTPC))
  ;[0 0 0] HitEvents
  ;;[1 1 1] If no enemy under cursor, set reference to enemy under cursor to self
  (Variables|/Game/Blueprints/ThirdPerson/Blueprints/BP_ThirdPersonCharacter.BP_ThirdPersonCharacter_C|GetCurrEnemyUnderCursor _tpc
    (:then)
    (:else
      (Variables|/Game/Blueprints/ThirdPerson/Blueprints/BP_ThirdPersonCharacter.BP_ThirdPersonCharacter_C|SetCurrEnemyUnderCursor _tpc self))))

(event OnEndCursorOver(Mesh)
  (params (TouchedComponent :type Primitive%20Component%20Object%20Reference))
  ;[0 0 0] HitEvents
  ;;[1 1 1] Set enemy under cursor to null upon leaving
  (bind _currenemyundercursor (Variables|/Game/Blueprints/ThirdPerson/Blueprints/BP_ThirdPersonCharacter.BP_ThirdPersonCharacter_C|GetCurrEnemyUnderCursor (Variables|Default|GetTPC))
    (:then
      (if (== _currenemyundercursor self)
        (Variables|/Game/Blueprints/ThirdPerson/Blueprints/BP_ThirdPersonCharacter.BP_ThirdPersonCharacter_C|SetCurrEnemyUnderCursor (Variables|Default|GetTPC) 0)))
    (:else)))

(event Custom|OnDead
  ;[0 0 0] HitEvents
  ;;[1 1 1] On dead, drop current Gift and update player's combo
  (if (not (Variables|/Game/Blueprints/Common/BPC_Character.BPC_Character_C|GetbIsDead (Variables|Default|GetBPC_Character)))
    (Default|CallAIDeadDispatcher)
    (Utilities|ConverttoRagdoll)
    (Game|SpawnActorfromClass "/Game/Blueprints/Actions/BP_Gift_DroppedPerm.BP_Gift_DroppedPerm_C" (Math|Transform|MakeTransform (Transformation|GetActorLocation) "0, 0, 0" "1.000000,1.000000,1.000000") "Undefined" 0 (Variables|Config|GetGiftSpecialty) 0)
    (Default|OnKillEnemy (Variables|Default|GetTPC))))

(event Custom|UnfreezeAnim
  ;[0 0 0] HitEvents
  ;;[1 1 1] Freeze
  (Class|TimelineComponent|SetIgnoreTimeDilation (Variables|Default|GetTimeline_Unfreeze) true)
  (bind _returnvalue (Rendering|Material|GetScalarParameterValue (Utilities|Array|Get(acopy) (Variables|Components|GetMaterialInstances)) "FreezeAmount" :!class /Script/Engine.MaterialInstanceDynamic))
  (bind _alpha (Timeline|Timeline_Unfreeze PlayFromStart)
    (:Update
      (Utility|UpdateMatParameter "FreezeAmount" (Math|Float|Lerp _returnvalue -1e+01 _alpha)))
    (:Finished
      (Variables|Default|SetCustomTimeDilation 1.0))))

(event Custom|AI_Attack
  (CallFunction|Attack)
  (Default|CallOnAttackFinished))

(event EventFreeze
  (params (Duration :type Float%20%28double-precision%29))
  ;[0 0 0] HitEvents
  ;;[1 1 1] Freeze
  (CallFunction|BeginFreeze Duration))

(event EventBeginPlay
  (CallFunction|InitializeVariables)
  (if (Utilities|Enum|NotEqual(Enum) (Variables|Config|GetGiftSpecialty) "NewEnumerator19")
    (Utilities|Time|SetTimerbyEvent (delegate Custom|AI_Attack) 2.0 true)))

(event EventSetStagger
  (params (bIsStagger :type Boolean))
  ;[0 0 0] HitEvents
  (Variables|/Game/Blueprints/Common/BPC_Character.BPC_Character_C|SetbIsStagger (Variables|Default|GetBPC_Character) bIsStagger))

(event EventTakeDamage
  (params (DamageInfo :type S%20Damage%20Info%20Structure))
  (bind (_damageamount _damageresponse) (Utilities|Struct|BreakS_DamageInfo DamageInfo))
  ;[0 0 0] HitEvents
  (if (not (Variables|/Game/Blueprints/Common/BPC_Character.BPC_Character_C|GetbIsDead (Variables|Default|GetBPC_Character)))
    (Default|TakeDamage (Variables|Default|GetBPC_Character) _damageamount _damageresponse)
    (CallFunction|OnDamaged DamageInfo)))

(fn ConstructionScript
  (EventDispatchers|BindEventtoOnDeath (Variables|Default|GetBPC_Character) (EventDispatchers|CreateEvent :!event Custom|OnDead)))

(fn UpdateMatParameter
  (params (ParameterName :type Name) (Value :type Float%20%28single-precision%29))
  (for _array_element (Variables|Components|GetMaterialInstances)
    (Rendering|Material|SetScalarParameterValue _array_element ParameterName Value :!class /Script/Engine.MaterialInstanceDynamic)))

(fn InitializeVariables
  (bind _aswb_enemy_hp (Utilities|Casting|CastToWB_EnemyHP (UserInterface|GetWidget (Variables|Default|GetHealthBar))))
  (bind _output_get (Variables|Components|SetWB%20Enemy%20HP _aswb_enemy_hp))
  (Widget|SetRenderOpacity _output_get 0.0)
  (Variables|/Game/Widgets/World/WB_EnemyHP.WB_EnemyHP_C|SetRef_Character _output_get (Variables|Default|GetBPC_Character))
  (bind _asbp_third_person_character (Utilities|Casting|CastToBP_ThirdPersonCharacter (Game|GetPlayerCharacter 0)))
  (Variables|Default|SetTPC _asbp_third_person_character)
  (Utilities|InitializeMaterialInstances))

(fn Attack
  (if (Utilities|Enum|Equal(Enum) (Utilities|Struct|BreakS_Gift_Type (.Gift%20Type (CallFunction|GetGiftOfSpecialty (Variables|Config|GetGiftSpecialty)))) "NewEnumerator0")
    (Default|CastGift (Variables|Default|GetBPC_Sera_Gift_Fireball))
    (else
      (Default|CastGift (Variables|Default|GetBPC_Sera_Gift_Frostbolt)))))

(fn AttackDetection0
  (bind _mesh (Variables|Character|GetMesh))
  (bind _outhit (Collision|SphereTraceForObjects (Transformation|GetSocketLocation _mesh "RightArm") (Transformation|GetSocketLocation _mesh "RightHandMiddle4") 3e+01 (Utilities|Array|MakeArray "ObjectTypeQuery3" "ObjectTypeQuery2") false 0 "None" true "(R=1.000000,G=0.000000,B=0.000000,A=1.000000)" "(R=0.000000,G=1.000000,B=0.000000,A=1.000000)" 1.0))
  (if (.bInitialOverlap (Collision|BreakHitResult _outhit))
    (Utilities|Casting|CastToBP_Sera_DodgeGhost (.HitActor (Collision|BreakHitResult _outhit))
      (:then
        (bind _asbp_third_person_character (Utilities|Casting|CastToBP_ThirdPersonCharacter (Game|GetPlayerCharacter 0)))
        (Default|ActivatePerfectDodge _asbp_third_person_character (Variables|Config|GetGiftSpecialty)))
      (:CastFailed
        (bind _asbp_third_person_character_2 (Utilities|Casting|CastToBP_ThirdPersonCharacter (.HitActor (Collision|BreakHitResult _outhit))))
        (if (not (Variables|/Game/Blueprints/ThirdPerson/Blueprints/BP_ThirdPersonCharacter.BP_ThirdPersonCharacter_C|GetbIsDodging _asbp_third_person_character_2))
          (Default|TakeDamage _asbp_third_person_character_2 (Utilities|Struct|MakeS_DamageInfo 0.5 (Transformation|GetWorldLocation (Variables|/Script/Engine.Character|GetCapsuleComponent _asbp_third_person_character_2)))))))))

(fn BeginFreeze
  (params (Duration :type Float%20%28double-precision%29))
  (if (not (Variables|/Game/Blueprints/Common/BPC_Character.BPC_Character_C|GetbIsDead (Variables|Default|GetBPC_Character)))
    (Utilities|Time|ClearandInvalidateTimerbyHandle (Variables|Actions|GetFreezeTimer))
    (Audio|Components|Audio|Stop (Variables|Default|GetTimeline_Unfreeze))
    (Utility|UpdateMatParameter "FreezeAmount" 1e+01)
    (Variables|Default|SetCustomTimeDilation 0.0)
    (bind _returnvalue (Utilities|Time|SetTimerbyEvent (EventDispatchers|CreateEvent :!event Custom|UnfreezeAnim) Duration))
    (Variables|Actions|SetFreezeTimer _returnvalue)))

(fn OnDamaged
  (params (DamageInfo :type S%20Damage%20Info%20Structure))
  (bind (_damageamount _damageresponse _damageelement _damagelocation) (Utilities|Struct|BreakS_DamageInfo DamageInfo))
  (bind _tpc (Variables|Default|GetTPC))
  (Default|AddDamagetoWindow (Variables|/Game/Blueprints/ThirdPerson/Blueprints/BP_ThirdPersonCharacter.BP_ThirdPersonCharacter_C|GetWB_DamageWindow (Variables|Default|GetTPC)) _damageamount _damageelement _damagelocation)
  ;[1 1 1] Report Damaged for AI
  (Class|AISenseDamage|ReportDamageEvent self _tpc _damageamount (Transformation|GetActorLocation _tpc) "0, 0, 0" "None")
  ;[1 1 1] Update HP Opacity
  (Widget|SetRenderOpacity (Variables|Components|GetWB%20Enemy%20HP) (Math|Float|SelectFloat 0.0 0.8 (Variables|/Game/Blueprints/Common/BPC_Character.BPC_Character_C|GetbIsDead (Variables|Default|GetBPC_Character)))))

(fn BeginSlide
  (params (bSlide :type Boolean) (SlidingSurface :type Actor%20Object%20Reference))
  (Default|BeginSlide (Variables|Default|GetBPC_Character) bSlide SlidingSurface)
  (return))

(fn GetCurrBeam
  (return (Variables|/Game/Blueprints/Common/BPC_Character.BPC_Character_C|GetCurrBeam (Variables|Default|GetBPC_Character))))

(fn GetCurrShield
  (return (Variables|/Game/Blueprints/Common/BPC_Character.BPC_Character_C|GetCurrShield (Variables|Default|GetBPC_Character))))

(fn GetHealth
  (return (Variables|/Game/Blueprints/Common/BPC_Character.BPC_Character_C|GetHealth (Variables|Default|GetBPC_Character))))

(fn GetIsDead
  (return (Variables|/Game/Blueprints/Common/BPC_Character.BPC_Character_C|GetbIsDead (Variables|Default|GetBPC_Character))))

(fn GetLocation
  (return (Transformation|GetActorLocation)))

(fn GetMaxHealth
  (return (Variables|/Game/Blueprints/Common/BPC_Character.BPC_Character_C|GetMaxHealth (Variables|Default|GetBPC_Character))))

(fn GetPatrolRoute
  (return (Variables|AI|GetPatrolRoute)))

(fn GetProjectileSpawnTransform
  (return (Math|Transform|MakeTransform (Transformation|GetSocketLocation (Variables|Character|GetMesh) "RightHand") (Math|Rotator|CombineRotators (Variables|/Script/Engine.SceneComponent|GetRelativeRotation (Variables|Character|GetMesh)) "0.000000,90.000000,0.000000") "1.000000,1.000000,1.000000")))

(fn GetProjectileTarget
  (bind _returnvalue (Game|GetPlayerCharacter 0))
  (return _returnvalue (Transformation|GetActorLocation _returnvalue)))

(fn GetRange
  (return 2.5e+02))

(fn GetShouldPlayCastAnim
  (return (not (AI|Components|NavMovement|IsFalling (Variables|Character|GetCharacterMovement)))))

(fn Heal
  (params (HealAmt :type Float%20%28double-precision%29))
  (bind _newhealth (Default|Heal (Variables|Default|GetBPC_Character) HealAmt))
  (return _newhealth))

(fn SetCastGiftType
  (params (CastGiftType :type E_Gift_CastType%20Enum :default "NewEnumerator0"))
  (Variables|/Game/Blueprints/Common/BPC_Character.BPC_Character_C|SetCastGiftType (Variables|Default|GetBPC_Character) CastGiftType)
  (return))

(fn SetCurrBeam
  (params (Beam :type BP%20Gift%20Beam%20Object%20Reference))
  (Variables|/Game/Blueprints/Common/BPC_Character.BPC_Character_C|SetCurrBeam (Variables|Default|GetBPC_Character) Beam)
  (return))

(fn SetCurrFiringGift
  (params (CurrFiringGift :type BPC%20Gift%20Base%20Object%20Reference))
  (Variables|/Game/Blueprints/Common/BPC_Character.BPC_Character_C|SetCurrFiringGift (Variables|Default|GetBPC_Character) CurrFiringGift)
  (return))

(fn SetCurrShield
  (params (Shield :type BP%20Gift%20Shield%20Object%20Reference))
  (Variables|/Game/Blueprints/Common/BPC_Character.BPC_Character_C|SetCurrShield (Variables|Default|GetBPC_Character) Shield)
  (return))

(fn SetMovementSpeed
  (params (SpeedType :type E_Enemy_MovementSpeed%20Enum :default "NewEnumerator0"))
  (bind _output_get (Variables|/Script/Engine.CharacterMovementComponent|SetMaxWalkSpeed (Variables|Character|GetCharacterMovement) (Utilities|Select :Index SpeedType :NewEnumerator0 0.0 :NewEnumerator1 2e+02 :NewEnumerator2 4e+02 :NewEnumerator3 6e+02)))
  (return _output_get))