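; BP_Rambit is an actor that rides as a child actor of the third-person character and can pause gameplay movement.
; Each Tick it rolls the Rambit component with the character's Y velocity and flips that roll and the yaw according to facing.
; PauseMovement toggles the player's movement lock and freezes all BP_Enemy actors through CustomTimeDilation.
; The dialogue start and end events switch on a function index but have no cases wired.
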(event EventOnStartDialogue
  (params (FunctionIndex :type Integer))
  (switch int FunctionIndex))

(event EventOnEndDialogue
  (params (FunctionIndex :type Integer))
  (switch int FunctionIndex))

(event EventTick
  (params (DeltaSeconds :type Float%20%28single-precision%29))
  (bind _returnvalue (Transformation|GetActorRotation))
  (bind _returnvalue_2 (>= (.yaw _returnvalue) 9e+01))
  ;[1 0.4453 0] Update rotations when rotating/moving player character
  (bind _tpc (Variables|Default|GetTPC)
    (:then
      (Transformation|SetRelativeRotation (Variables|Default|GetRambit) (Math|Rotator|MakeRotator (Math|Float|MapRangeClamped (* (.y (Transformation|GetVelocity _tpc)) (Math|Float|SelectFloat -1.0 1.0 _returnvalue_2)) -6e+02 6e+02 -15.0 15.0) 0.0 (Math|Float|SelectFloat -4e+01 4e+01 _returnvalue_2)) false false))
    (:else)))

(event EventBeginPlay
  (bind _asbp_third_person_character (Utilities|Casting|CastToBP_ThirdPersonCharacter (Actor|GetParentActor)))
  (Variables|Default|SetTPC _asbp_third_person_character))

(fn ConstructionScript)

(fn PauseMovement
  (params (bPause :type Boolean))
  (Variables|/Game/Blueprints/ThirdPerson/Blueprints/BP_ThirdPersonCharacter.BP_ThirdPersonCharacter_C|SetbDisableMovement (Variables|Default|GetTPC) bPause)
  (bind _outactors (Actor|GetAllActorsOfClass "/Game/Blueprints/Enemy/BP_Enemy.BP_Enemy_C"))
  (for _array_element _outactors
    (Variables|/Script/Engine.Actor|SetCustomTimeDilation _array_element (Math|Float|SelectFloat 0.0 1.0 bPause))))