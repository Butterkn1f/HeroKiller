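; Swingable world rope that the third-person character grabs on overlapping its box, sized from CableLength at construction.
; Grabbing attaches the sphere to the left hand and starts a looping timer that applies radial-velocity-opposing force and splits length between two cables at the player.
; Release launches the character upward, except when overstretching forces it.
; A timeline then eases sphere, cables and box back to rest.
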(event OnComponentBeginOverlap(Box)
  (params (OverlappedComponent :type Primitive%20Component%20Object%20Reference) (OtherActor :type Actor%20Object%20Reference) (OtherComp :type Primitive%20Component%20Object%20Reference) (OtherBodyIndex :type Integer) (bFromSweep :type Boolean) (SweepResult :type Hit%20Result%20Structure%20%28by%20ref%29))
  (bind _asbp_third_person_character (Utilities|Casting|CastToBP_ThirdPersonCharacter OtherActor))
  (Variables|Default|SetTPC _asbp_third_person_character)
  (CallFunction|AttachPlayertoRope))

(event Custom|OnReleaseRope
  (params (bDisableLaunch :type Boolean))
  (bind _tpc (Variables|Default|GetTPC))
  (bind _mesh (Variables|/Script/Engine.Character|GetMesh _tpc))
  (bind _returnvalue (Transformation|GetWorldRotation _mesh))
  (Utilities|Time|ClearandInvalidateTimerbyHandle (Variables|Default|GetSwingPlayerTimer))
  (Default|UpdateCurrRope (Variables|Default|GetTPC))
  (Transformation|DetachFromComponent (Variables|Default|GetSphere) "KeepWorld" "KeepWorld" "KeepWorld" true)
  (CallFunction|MoveBackSphere (Transformation|GetWorldLocation (Variables|Default|GetSphere)) (Variables|/Script/CableComponent.CableComponent|GetCableLength (Variables|Default|GetFirstHalfCable)) (Variables|/Script/CableComponent.CableComponent|GetCableLength (Variables|Default|GetSecondHalfCable)))
  (if (not bDisableLaunch)
    (Character|LaunchCharacter _tpc (+ (Transformation|GetVelocity _tpc) "0.000000,0.000000,1000.000000") true true)
    (Default|TimelineEventRotateBodytoTarget _tpc (Math|Rotator|MakeRotator 0.0 (.pitch _returnvalue) (.yaw _returnvalue)))))

(event Custom|MoveBackSphere
  (params (InitialPos :type Vector) (CurrFirstCableLength :type Float%20%28double-precision%29) (CurrSecondCableLength :type Float%20%28double-precision%29))
  (bind _returnvalue (Transformation|GetActorLocation))
  (bind _box (Variables|Default|GetBox))
  (bind _sphere (Variables|Default|GetSphere))
  (bind _relativelocation (Variables|/Script/Engine.SceneComponent|GetRelativeLocation _sphere))
  (bind (_direction _x _alpha) (Timeline|Timeline_MoveBack PlayFromStart)
    (:Update
      (Transformation|SetWorldLocation (Variables|Default|GetSphere) (Math|Vector|MakeVector (Math|Float|Lerp (.x InitialPos) 0.0 _x) (Math|Float|Lerp (.y InitialPos) (.y _returnvalue) _alpha) (Math|Float|Lerp (.z InitialPos) (- (.z _returnvalue) (Variables|Config|GetCableLength)) _alpha)) false true)
      (Variables|/Script/CableComponent.CableComponent|SetCableLength (Variables|Default|GetFirstHalfCable) (Math|Float|Lerp CurrFirstCableLength (Variables|Config|GetCableLength) _alpha))
      (Transformation|SetRelativeLocation _box (Math|Vector|MakeVector 0.0 0.0 (Math|Float|Lerp CurrFirstCableLength (Variables|Config|GetCableLength) _alpha)) false true)
      (Components|Box|SetBoxExtent _box (Math|Vector|MakeVector 15.0 15.0 (* (Math|Float|Lerp CurrFirstCableLength (Variables|Config|GetCableLength) _alpha) 0.5)) true)
      (Variables|/Script/CableComponent.CableComponent|SetCableLength (Variables|Default|GetSecondHalfCable) (Math|Float|Lerp CurrSecondCableLength 0.0 _alpha))
      (Transformation|SetWorldRotation (Variables|Default|GetSphere) (Math|Rotator|FindLookatRotation (Math|Vector|MakeVector 0.0 (.y _relativelocation) (.z _relativelocation)) (Math|Vector|VectorZero)) false false))
    (:Finished
      (Transformation|SetWorldRotation (Variables|Default|GetSphere) "0, 0, 0" false false))))

(fn ConstructionScript
  (bind _box (Variables|Default|GetBox))
  (Variables|/Script/CableComponent.CableComponent|SetCableLength (Variables|Default|GetFirstHalfCable) (Variables|Config|GetCableLength))
  (Transformation|SetRelativeLocation (Variables|Default|GetSphere) (* (Variables|Config|GetCableLength) "0.000000,0.000000,-1.000000") false true)
  (Transformation|SetRelativeLocation _box (Math|Vector|MakeVector 0.0 0.0 (Variables|Config|GetCableLength)) false true)
  (Components|Box|SetBoxExtent _box (Math|Vector|MakeVector 15.0 15.0 (* (Variables|Config|GetCableLength) 0.5)) true)
  (Variables|/Script/CableComponent.CableComponent|SetEndLocation (Variables|Default|GetSecondHalfCable) (Math|Vector|MakeVector 0.0 0.0 (Variables|Config|GetCableLength))))

(fn AttachPlayertoRope
  (bind _bropeupdated (Default|UpdateCurrRope (Variables|Default|GetTPC) self))
  (if _bropeupdated
    (Transformation|AttachComponentToComponent (Variables|Default|GetSphere) (Variables|/Script/Engine.Character|GetMesh (Variables|Default|GetTPC)) "LeftHand" "SnapToTarget" "KeepWorld" "KeepWorld" false)
    (bind _returnvalue (Utilities|Time|SetTimerbyFunctionName 0 "SwingPlayer" 0.01 true))
    (Variables|Default|SetSwingPlayerTimer _returnvalue)))

(fn SwingPlayer
  (bind _returnvalue (Transformation|GetActorLocation))
  (bind _self self)
  (bind _tpc (Variables|Default|GetTPC))
  (bind _tpc_2 (Variables|Default|GetTPC))
  (bind _returnvalue_2 (Transformation|GetActorLocation _tpc))
  (bind _returnvalue_3 (Transformation|GetDistanceTo _tpc_2 _self))
  (bind _returnvalue_4 (- _returnvalue_2 _returnvalue))
  (Physics|AddForce (Variables|/Script/Engine.Character|GetCharacterMovement (Variables|Default|GetTPC)) (* (* (Math|Vector|DotProduct (Transformation|GetVelocity _tpc) _returnvalue_4) (Math|Vector|Normalize _returnvalue_4)) -2.0))
  (if (> (- (Variables|Config|GetCableLength) _returnvalue_3) 0.0)
    (Variables|/Script/CableComponent.CableComponent|SetCableLength (Variables|Default|GetFirstHalfCable) _returnvalue_3)
    (Variables|/Script/CableComponent.CableComponent|SetCableLength (Variables|Default|GetSecondHalfCable) (- (Variables|Config|GetCableLength) _returnvalue_3))
    (else
      (CallFunction|OnReleaseRope true))))