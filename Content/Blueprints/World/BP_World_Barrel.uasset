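; BP_World_Barrel is a destructible Chaos Geometry Collection barrel that explodes when it breaks.
; On break, it activates particles and a radial force, then sphere-traces nearby pawns and sends damage messages, dealing less to BP_ThirdPersonCharacter.
; A timeline can sink and shrink the remains before destroying the actor, but its trigger is disconnected and the fragment-removal event is empty.
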(event OnChaosBreakEvent(GeometryCollection)
  (params (BreakEvent :type Chaos%20Break%20Event%20Structure%20%28by%20ref%29))
  (bind _returnvalue (Transformation|GetActorLocation))
  (Components|Activation|Activate (Variables|Default|GetParticleSystem) true)
  (bind _outhits (Collision|MultiSphereTraceForObjects _returnvalue _returnvalue 3e+02 (Utilities|Array|MakeArray "ObjectTypeQuery3") false 0 "None"))
  (for _array_element _outhits
    (Class|BPICharacter|TakeDamage(Message) (.HitActor (Collision|BreakHitResult _array_element)) (Utilities|Struct|MakeS_DamageInfo (Math|Float|SelectFloat 8e+01 1e+02 (== (Utilities|GetClass (.HitActor (Collision|BreakHitResult _array_element))) "/Game/Blueprints/ThirdPerson/Blueprints/BP_ThirdPersonCharacter.BP_ThirdPersonCharacter_C")) "NewEnumerator1" "NewEnumerator0" _returnvalue "NewEnumerator3")))
  (Components|Activation|Activate (Variables|Default|GetRadialForce) true))

(event OnChaosRemovalEvent(GeometryCollection)
  (params (RemovalEvent :type Chaos%20Removal%20Event%20Structure%20%28by%20ref%29))
  ;[1 1 1] Each time a fragment despawns, we add it to the total broken mass. Once the total removed exceeds a value, we just destroy the entire actor.
  ; This is due to the anchor always holding onto a small piece of the destructible, so we use this to automatically destroy it.
)

(event Custom|TimelineEvent_ScaleDown
  (bind _geometrycollection (Variables|Default|GetGeometryCollection))
  ;[1 1 1] Simulate same animation as default removal of fragment
  (bind _alpha (Timeline|Timeline PlayFromStart)
    (:Update
      (Transformation|SetRelativeTransform _geometrycollection (Math|Transform|MakeTransform (+ (Variables|/Script/Engine.SceneComponent|GetRelativeLocation _geometrycollection) (Math|Vector|MakeVector 0.0 0.0 (Math|Float|Lerp 0.0 -15.0 _alpha))) "0, 0, 0" (Math|Vector|Lerp(Vector) "1.000000,1.000000,1.000000" "0, 0, 0" _alpha)) false false))
    (:Finished
      (Actor|DestroyActor))))

(fn ConstructionScript)