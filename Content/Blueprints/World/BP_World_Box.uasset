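; BP_World_Box is a world box actor built on a Geometry Collection component that removes itself once enough of it has been destroyed.
; Chaos removal events add the mass of removed pieces to a running broken-mass total.
; When that total passes a fixed threshold, it destroys the Geometry Collection component once, then destroys the actor after a brief delay.
; The crumbling event is bound but empty.
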(event OnChaosCrumblingEvent(GeometryCollectionComponent)
  (params (CrumbleEvent :type Chaos%20Crumbling%20Event%20Structure%20%28by%20ref%29)))

(event OnChaosRemovalEvent(GeometryCollectionComponent)
  (params (RemovalEvent :type Chaos%20Removal%20Event%20Structure%20%28by%20ref%29))
  (bind _output_get (Variables|Default|SetBrokenMass (+ (Variables|Default|GetBrokenMass) (Utilities|Struct|BreakChaosRemovalEvent RemovalEvent))))
  (if (> _output_get 4.8e+03)
    (Utilities|FlowControl|DoOnce false
      (:Completed
        (Components|DestroyComponent (Variables|Default|GetGeometryCollectionComponent))
        (Utilities|FlowControl|Delay 0.02)
        (Actor|DestroyActor)))))

(fn ConstructionScript)