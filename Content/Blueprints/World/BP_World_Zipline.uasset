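; Zipline actor that carries BP_ThirdPersonCharacter between its Start and End points.
; The construction script fits a spline to both points and adds a spline mesh beneath it as the overlap trigger.
; On overlap, it picks the far end by world Y, aligns the character's height and mesh rotation, then a looping timer drives velocity along world Y.
; Riders release near the target without a launch; OnReleaseZipline can otherwise launch them upward.
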(event Custom|OnComponentBeginOverlap_Event
  (params (OverlappedComponent :type Primitive%20Component%20Object%20Reference) (OtherActor :type Actor%20Object%20Reference) (OtherComp :type Primitive%20Component%20Object%20Reference) (OtherBodyIndex :type Integer) (bFromSweep :type Boolean) (SweepResult :type Hit%20Result%20Structure%20%28by%20ref%29))
  (bind _asbp_third_person_character (Utilities|Casting|CastToBP_ThirdPersonCharacter OtherActor))
  (bind _output_get (Variables|Default|SetTPC _asbp_third_person_character))
  (bind _bziplineupdated (Default|UpdateCurrZipline _output_get self))
  (if _bziplineupdated
    (bind (_targetrot _targetendloc _direction) (CallFunction|GetZipDirection (Transformation|GetActorLocation (Variables|Default|GetTPC))))
    (Variables|Default|SetTarget%20End%20Loc _targetendloc)
    (Variables|Default|SetCurrDirection _direction)
    (Utilities|FlowControl|Delay 0.1)
    (Transformation|SetActorLocation (Variables|Default|GetTPC) (Math|Vector|MakeVector (.X (Math|Vector|BreakVector (Transformation|GetActorLocation (Variables|Default|GetTPC)))) (.Y (Math|Vector|BreakVector (Transformation|GetActorLocation (Variables|Default|GetTPC)))) (- (.z (Transformation|GetActorLocation)) (Class|KismetAnimationLibrary|DistanceBetweenTwoSocketsandMapRange (Variables|/Script/Engine.Character|GetMesh (Variables|Default|GetTPC)) "RightHand" "RTS_World" "Hips" "RTS_World" false 0.0 0.0 0.0 0.0))) false true)
    (Transformation|SetRelativeRotation (Variables|/Script/Engine.Character|GetMesh (Variables|Default|GetTPC)) _targetrot false false)
    (bind _returnvalue (Utilities|Time|SetTimerbyFunctionName 0 "UpdatePlayerVelocity" 0.01 true))
    (Variables|Default|SetZiplineTimer _returnvalue)))

(event Custom|OnReleaseZipline
  (params (bDisableLaunch :type Boolean))
  (bind _tpc (Variables|Default|GetTPC))
  (Utilities|Time|ClearandInvalidateTimerbyHandle (Variables|Default|GetZiplineTimer))
  (Default|UpdateCurrZipline (Variables|Default|GetTPC))
  (if (not bDisableLaunch)
    (Character|LaunchCharacter _tpc (+ (Transformation|GetVelocity _tpc) "0.000000,0.000000,1000.000000") true true)))

(event Custom|OnComponentEndOverlap_Event
  (params (OverlappedComponent :type Primitive%20Component%20Object%20Reference) (OtherActor :type Actor%20Object%20Reference) (OtherComp :type Primitive%20Component%20Object%20Reference) (OtherBodyIndex :type Integer)))

(event EventBeginPlay
  (bind _cablecollision (Variables|Components|GetCableCollision))
  (Collision|AssignOnComponentBeginOverlap _cablecollision (delegate Custom|OnComponentBeginOverlap_Event))
  (Collision|AssignOnComponentEndOverlap _cablecollision (delegate Custom|OnComponentEndOverlap_Event)))

(fn ConstructionScript
  (bind _splinecollision (Variables|Default|GetSplineCollision))
  (bind _splinecollision_2 (Variables|Default|GetSplineCollision))
  (bind _splinecollision_3 (Variables|Default|GetSplineCollision))
  ;[1 1 1] Set zipline end point
  (Spline|SetLocationatSplinePoint _splinecollision 0 (Transformation|GetWorldLocation (Variables|Default|GetStart)) "World" true)
  (Spline|SetLocationatSplinePoint _splinecollision 1 (Transformation|GetWorldLocation (Variables|Default|GetEnd)) "World" true)
  ;[1 1 1] Set collision
  (for _index (range 0 (- (Spline|GetNumberOfSplinePoints _splinecollision) 2))
    (bind _returnvalue (AddComponent|AddSplineMeshComponent false))
    (bind _output_get (Variables|Components|SetCableCollision _returnvalue))
    (SplineMesh|SetStartandEnd _output_get (- (Spline|GetLocationatSplinePoint _splinecollision_3 _index "Local") "0.000000,0.000000,50.000000") (Spline|GetTangentatSplinePoint _splinecollision_3 _index "Local") (- (Spline|GetLocationatSplinePoint _splinecollision_2 (+ _index 1) "Local") "0.000000,0.000000,50.000000") (Spline|GetTangentatSplinePoint _splinecollision_2 (+ _index 1) "Local") true :!class /Script/Engine.SplineMeshComponent)))

(fn GetZipDirection
  (params (ActorLocation :type Vector))
  (bind _start (Variables|Default|GetStart))
  (bind _returnvalue (Transformation|GetWorldLocation _start))
  (if (> (.Y (Class|KismetMathLibrary|BreakVector3f ActorLocation)) (+ (.Y (Class|KismetMathLibrary|BreakVector3f _returnvalue)) (* (Math|Vector|Distance(Vector) _returnvalue (Transformation|GetWorldLocation (Variables|Default|GetEnd))) 0.5)))
    (return "0.000000,180.000000,0.000000" (Transformation|GetWorldLocation (Variables|Default|GetStart)) 0)
    (else
      (return "0.000000,0.000000,0.000000" (Transformation|GetWorldLocation (Variables|Default|GetEnd)) 1))))

(fn UpdatePlayerVelocity
  (bind _tpc (Variables|Default|GetTPC)
    (:then
      (Variables|/Script/Engine.MovementComponent|SetVelocity (Variables|/Script/Engine.Character|GetCharacterMovement _tpc) (Utilities|Select :Index (Variables|Default|GetCurrDirection) :Option%200 "0.000000,-1000.000000,0.000000" :Option%201 "0.000000,1000.000000,0.000000"))
      (if (<= (Class|KismetMathLibrary|VectorDistanceSquared (Transformation|GetActorLocation _tpc) (Variables|Default|GetTarget%20End%20Loc)) 2.5e+05)
        (CallFunction|OnReleaseZipline true)))
    (:else)))