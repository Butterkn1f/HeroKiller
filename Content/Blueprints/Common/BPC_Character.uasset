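; BPC_Character is a character component Blueprint that tracks health and death state.
; TakeDamage and Heal adjust Health within a fixed clamped range, and Heal returns the new value.
; At zero health, TakeDamage calls the OnDeath dispatcher and then sets IsDead, with no guard against firing again on later hits.
; Its DamageResponse input is unused, Heal never clears IsDead, and the event graph is empty.
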(event EventBeginPlay)

(event EventTick
  (params (DeltaSeconds :type Float%20%28single-precision%29)))

(fn TakeDamage
  (params (DamageAmount :type Float%20%28double-precision%29) (DamageResponse :type E_DamageResponse%20Enum :default "NewEnumerator0"))
  (bind _output_get (Variables|Stats|SetHealth (Math|Float|Clamp(Float) (- (Variables|Stats|GetHealth) DamageAmount) 0.0 1e+02)))
  (if (== _output_get 0.0)
    (Default|CallOnDeath)
    (Variables|SpecialMovement|SetbIsDead true)))

(fn Heal
  (params (HealAmt :type Float%20%28double-precision%29))
  (bind _output_get (Variables|Stats|SetHealth (Math|Float|Clamp(Float) (+ HealAmt (Variables|Stats|GetHealth)) 0.0 1e+02)))
  (return _output_get))