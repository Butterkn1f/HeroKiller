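; BP_AudioManager handles level background music, switching between a normal track and a paused variant.
; On BeginPlay it picks the track pair by level name for the tutorial or first boss map and starts the normal track.
; Playback percent events from both tracks record the current position in seconds.
; SetPauseBGM pauses one track and fades in the other slightly ahead of that position, keeping the music roughly continuous.
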(event Custom|SetPauseBGM
  (params (bPaused :type Boolean))
  (bind _bgm (Variables|Default|GetBGM))
  (bind _bgmpaused (Variables|Default|GetBGMPaused))
  (bind _returnvalue (select bPaused _bgmpaused _bgm))
  (Class|AudioComponent|SetPaused (select bPaused _bgm _bgmpaused) true)
  (Audio|Components|Audio|FadeIn _returnvalue 0.5 1.0 (+ (Variables|Default|GetCurrBGMPosition) 0.5) "Linear" :!class /Script/Engine.AudioComponent)
  (Class|AudioComponent|SetPaused _returnvalue false))

(event Custom|OnAudioPlaybackPercent_Event
  (params (PlayingSoundWave :type Sound%20Wave%20Object%20Reference) (PlaybackPercent :type Float%20%28single-precision%29))
  (Variables|Default|SetCurrBGMPosition (* PlaybackPercent (Variables|/Script/Engine.SoundBase|GetDuration PlayingSoundWave))))

(event EventBeginPlay
  (bind _returnvalue (Game|GetCurrentLevelName true))
  (switch string _returnvalue
    (:M_00_TutorialMap
      (bind _returnvalue_2 (Audio|CreateSound2D "/Game/Audio/BGM/BGM_Tutorial.BGM_Tutorial" 1.0 1.0 0.0 0))
      (Variables|Default|SetBGM _returnvalue_2)
      (bind _returnvalue_3 (Audio|CreateSound2D "/Game/Audio/BGM/BGM_Tutorial_Paused.BGM_Tutorial_Paused" 1.0 1.0 0.0 0))
      (Variables|Default|SetBGMPaused _returnvalue_3))
    (:M_03_Boss1
      (bind _returnvalue_4 (Audio|CreateSound2D "/Game/Audio/BGM/BGM_Boss.BGM_Boss" 1.0 1.0 0.0 0))
      (Variables|Default|SetBGM _returnvalue_4)
      (bind _returnvalue_5 (Audio|CreateSound2D "/Game/Audio/BGM/BGM_Boss_Paused.BGM_Boss_Paused" 1.0 1.0 0.0 0))
      (Variables|Default|SetBGMPaused _returnvalue_5)))
  (Audio|Components|Audio|Play (Variables|Default|GetBGM) 0.0)
  (EventDispatchers|AssignOnAudioPlaybackPercent (Variables|Default|GetBGM) (delegate Custom|OnAudioPlaybackPercent_Event)))

(fn ConstructionScript)